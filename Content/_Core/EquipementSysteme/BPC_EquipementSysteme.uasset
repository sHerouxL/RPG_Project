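; Player component that handles weapon pickup and the equipment menu.
; On Interact, a sphere trace from the follow camera finds a BP_WeaponTest, appends its item data to WeaponSlots and destroys the actor.
; The menu input toggles the WBP_Equipement widget, switching cursor and input mode, and blocks attacks through the attack component and freezes movement while open.
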(event `self.ReceiveBeginPlay`
  ;[0.05098 0.0483 0.001245] Begin play
  (bind _asbp_player (cast `/Game/_GameMain/RPJ_Player/BP_Player` (`self.GetOwner`)))
  (set `self.Follow Camera` (`/Game/_GameMain/RPJ_Player/BP_Player.FollowCamera` _asbp_player))
  (set `self.BPC Attack Systeme` (`/Game/_GameMain/RPJ_Player/BP_Player.BPC_AttackSystem` _asbp_player)))

(event `EnhancedInput|/Game/ThirdPerson/Input/Actions/IA_Interact`
  (params (ActionValue :type Boolean) (ElapsedSeconds :type "Float (double-precision)") (TriggeredSeconds :type "Float (double-precision)") (InputAction :type "InputAction Object Reference" :default "/Game/ThirdPerson/Input/Actions/IA_Interact.IA_Interact"))
  (bind _follow_camera (`self.Follow Camera`))
  (bind _returnvalue (`SceneComponent.K2_GetComponentLocation` _follow_camera))
  ;[0.05127 0.05127 0.05127] GrabItem
  (:`Started`
    (bind (_outhit _returnvalue_2) (`KismetSystemLibrary.SphereTraceSingleForObjects` :`Start` _returnvalue :`End` (+ _returnvalue (* (`KismetMathLibrary.GetForwardVector` (`SceneComponent.K2_GetComponentRotation` _follow_camera)) 1000.0)) :`Radius` 15.0 :`ObjectTypes` (`|MakeArray` "ObjectTypeQuery2" :!type "EObjectTypeQuery Enum") :`DrawDebugType` "ForDuration"))
    (if _returnvalue_2
      (bind (_bblockinghit _binitialoverlap _time _distance _location _impactpoint _normal _impactnormal _physmat _hitactor) (`GameplayStatics.BreakHitResult` _outhit))
      ;;[0.05098 0.002389 0.008662] Comment
      (bind _asbp_weapon_test (cast `/Game/_Core/EquipementSysteme/BP_WeaponTest` _hitactor))
      (`self.AddWeapon` (`/Game/_Core/EquipementSysteme/BP_WeaponTest.ItemData` _asbp_weapon_test))
      (`Actor.K2_DestroyActor` _hitactor)
      (`KismetSystemLibrary.PrintString` "item gather"))))

(event `EnhancedInput|/Game/ThirdPerson/Input/Actions/IA_EquipementMenu`
  (params (ActionValue :type Boolean) (ElapsedSeconds :type "Float (double-precision)") (TriggeredSeconds :type "Float (double-precision)") (InputAction :type "InputAction Object Reference" :default "/Game/ThirdPerson/Input/Actions/IA_EquipementMenu.IA_EquipementMenu"))
  (bind _returnvalue (`GameplayStatics.GetPlayerController` 0))
  (bind _returnvalue_2 (`self.GetOwner`))
  ;[0.05098 0.0483 0.001245] Equipement menu panel
  (:`Started`
    (if (not (`self.IsPanelOpen?`))
      (set `/Game/_Core/Utils/BPC_AttackSystem.CanAttack?` false (`self.BPC Attack Systeme`))
      (bind _returnvalue_3 (`|CreateWidget` "/Game/_Core/Weapon/UI_Equipement/WBP_Equipement.WBP_Equipement_C"))
      (bind _output_get (set `self.EquipementWidget` _returnvalue_3))
      (`UserWidget.AddToViewport` _output_get 0)
      (set `PlayerController.bShowMouseCursor` true _returnvalue)
      (`WidgetBlueprintLibrary.SetInputMode_GameAndUIEx` _returnvalue (`self.EquipementWidget`))
      (bind _asbp_player (cast `/Game/_GameMain/RPJ_Player/BP_Player` _returnvalue_2))
      (`CharacterMovementComponent.SetMovementMode` (`Character.CharacterMovement` _asbp_player) "MOVE_None" 0)
      (set `self.IsPanelOpen?` true)
      (else
        (set `/Game/_Core/Utils/BPC_AttackSystem.CanAttack?` true (`self.BPC Attack Systeme`))
        (bind _equipementwidget (`self.EquipementWidget`)
          (:`then`
            (`Widget.RemoveFromParent` _equipementwidget)
            (set `self.EquipementWidget` null)
            (set `PlayerController.bShowMouseCursor` false _returnvalue)
            (`WidgetBlueprintLibrary.SetInputMode_GameOnly` _returnvalue)
            (bind _asbp_player_2 (cast `/Game/_GameMain/RPJ_Player/BP_Player` _returnvalue_2))
            (`CharacterMovementComponent.SetMovementMode` (`Character.CharacterMovement` _asbp_player_2) "MOVE_Walking" 0)
            (set `self.IsPanelOpen?` false))
          (:`else`))))))

(fn `AddWeapon`
  (params (NewItem :type "/Game/_Core/EquipementSysteme/S_Slots Structure (by ref)"))
  (`KismetArrayLibrary.Array_Add` (`self.WeaponSlots`) NewItem))