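; Arrow projectile actor that sticks into whatever actor it overlaps and plays a Sparrow hit effect.
; On Box overlap with another actor, it halts ProjectileMovement, zeroes gravity and attaches to that actor, keeping its world transform.
; It then disables Box collision and spawns an enlarged particle burst at the Box location.
; The graph applies no damage.
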(event `self.Box.OnComponentBeginOverlap`
  (params (OverlappedComponent :type "PrimitiveComponent Object Reference") (OtherActor :type "Actor Object Reference") (OtherComp :type "PrimitiveComponent Object Reference") (OtherBodyIndex :type Integer) (bFromSweep :type Boolean) (SweepResult :type "HitResult Structure (by ref)"))
  (bind _projectilemovement (`self.ProjectileMovement`))
  (if (!= OtherActor self)
    (`MovementComponent.StopMovementImmediately` _projectilemovement)
    (set `ProjectileMovementComponent.ProjectileGravityScale` 0.0 _projectilemovement)
    (`self.K2_AttachToActor` OtherActor "None" "KeepWorld" "KeepWorld" "KeepWorld")
    (`PrimitiveComponent.SetCollisionEnabled` (`self.Box`) "NoCollision")
    (`GameplayStatics.SpawnEmitterAtLocation` "/Game/_Core/VFX/P_Sparrow_HitHero.P_Sparrow_HitHero" (`SceneComponent.K2_GetComponentLocation` (`self.Box`)) (struct) (2.0 2.0 2.0))))

(fn `UserConstructionScript`)