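; BP_Gun is a weapon Blueprint with two fire modes: repeating projectiles and a box-trace flamethrower.
; Projectile fire spawns BP_Projectile at the Arrow on a looping timer set by ProjectilePerSeconde, playing a 2D sound cue with a Type parameter.
; StartFiring runs a Timeline that drives the length of debug-drawn box traces along the Arrow's forward vector until StopFiring.
; The trace results are unused, so the flamethrower applies no effect here.
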(event `StartFiringProjectiles`
  ;[0.01514 0.000851 0.03472] Tire des projectiles repeté en fonction du temps ici 1/8
  (`self.FireOneProjectile`)
  (`KismetSystemLibrary.K2_SetTimer` null "FireOneProjectile" (/ 1.0 (`self.ProjectilePerSeconde`)) true))

(event `FireOneProjectile`
  ;[0.01514 0.000851 0.03472] Fait apparaitre projectile sur canon gun
  (`|SpawnActorFromClass` "/Game/_Core/Weapon/MeleWeapon/BP_Projectile.BP_Projectile_C" (`SceneComponent.K2_GetComponentToWorld` (`self.Arrow`)) "Undefined" "MultiplyWithRoot" null null)
  ;[0.01514 0.000851 0.03472] Joue un son en fonctio0n de la valeur du parametre type
  (bind _returnvalue (`GameplayStatics.SpawnSound2D` "/Game/_TopDownShooter/Ressource/Ressources/Audio/A_FireProjectile_Cue.A_FireProjectile_Cue" 1.0 1.0 0.0 null))
  (`AudioParameterControllerInterface.SetIntParameter` _returnvalue "Type" 1))

(event `StopFiringProjeciles`
  ;[0.01514 0.000851 0.03472] arreter timer du tir
  (`KismetSystemLibrary.K2_ClearTimer` null "FireOneProjectile"))

(event `StartFiring`
  (bind _arrow (`self.Arrow`))
  (bind _returnvalue (`SceneComponent.K2_GetComponentLocation` _arrow))
  ;[1 0 0.01161] BOX TRACE POUR LE FLAME THROWER
  (bind (_direction _newtrack_0) (`Timeline|Timeline` :!via `PlayFromStart` :!label _label)
    (:`Update`
      (bind _output_get (set `self.FireLength` _newtrack_0))
      (`KismetSystemLibrary.BoxTraceSingle` :`Start` _returnvalue :`End` (+ _returnvalue (* (`SceneComponent.GetForwardVector` _arrow) _output_get)) :`HalfSize` (50.0 20.0 10.0) :`TraceChannel` "TraceTypeQuery1" :`DrawDebugType` "ForDuration" :`TraceColor` (struct :`R` 0.026972 :`G` 0.038052 :`B` 1.0 :`A` 1.0) :`DrawTime` 0.2))))

(event `StopFiring`
  ;[1 0 0.01161] BOX TRACE POUR LE FLAME THROWER
  (goto _label :!via `Stop`))

(fn `UserConstructionScript`)