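; BP_Projectile is a projectile actor that damages non-Hero actors and triggers physics field effects on impact.
; On a blocking hit, it spawns an effect along the surface normal and fires a temporary FS_MasterField, destroyed immediately after triggering.
; On overlap, it applies damage through BPI_Dammagable, ignoring damageable Hero-tagged actors.
; Other overlaps, damageable or not, play an impact sound and destroy the projectile.
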(event `self.ProjectileCollision.OnComponentHit`
  (params (HitComponent :type "PrimitiveComponent Object Reference") (OtherActor :type "Actor Object Reference") (OtherComp :type "PrimitiveComponent Object Reference") (NormalImpulse :type "Vector Structure") (Hit :type "HitResult Structure (by ref)"))
  (bind (_bblockinghit _binitialoverlap _time _distance _location _impactpoint _normal _impactnormal) (`GameplayStatics.BreakHitResult` Hit))
  (`NiagaraFunctionLibrary.SpawnSystemAtLocation` null _location (`KismetMathLibrary.Conv_VectorToRotator` _impactnormal))
  (bind _returnvalue (`|SpawnActorFromClass` "/Engine/EditorResources/FieldNodes/FS_MasterField.FS_MasterField_C" (`KismetMathLibrary.Conv_VectorToTransform` _location) "Undefined" "MultiplyWithRoot" null null))
  (`KismetSystemLibrary.PrintString` "ON A UN HIT !!!!!!!!!!" true true (struct :`R` 0.083899 :`G` 1.0 :`B` 0.119088 :`A` 1.0) 4.0)
  ;[1 1 1] Force field
  (`/Engine/EditorResources/FieldNodes/FS_MasterField.CE_Trigger` _returnvalue) ; pour exploser immediatement
  (`self.K2_DestroyActor` _returnvalue))

(event `self.ReceiveActorBeginOverlap`
  (params (OtherActor :type "Actor Object Reference"))
  ;[0.01338 0.01144 0.1198] Gerer les degats aux ennemy
  (if (`KismetSystemLibrary.DoesImplementInterface` OtherActor "/Game/_Core/Utils/BPI_Dammagable.BPI_Dammagable_C")
    (if (not (`self.ActorHasTag` OtherActor "Hero"))
      (message `/Game/_Core/Utils/BPI_Dammagable.AffectHealth(OLD)` OtherActor (`self.DammageAmount`))
      (`GameplayStatics.SpawnSoundAtLocation` "/Game/_TopDownShooter/Ressource/Ressources/Audio/A_ProjectileImpact_Cue.A_ProjectileImpact_Cue" (`self.K2_GetActorLocation`) (struct) 1.0 1.0 0.0 null null :!label _label)
      (`self.K2_DestroyActor`))
    (else
      (goto _label))))

(fn `UserConstructionScript`)