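; Mage enemy character that provides ground smash, basic spell, barrage, teleport and self-heal actions, plus its own speeds and ideal combat ranges.
; Attacks pass montage and damage info to BPCAttack.
; Teleport is a fast flying AI move with the mesh hidden and pawn collision ignored, restored on arrival or failure.
; Healing spawns a traced AOE that restores a share of max health per tick; teleport and heal both broadcast completion.
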(event `GroundSmashAttack`
  (params (AttackTarget :type "Actor Object Reference"))
  ;[0.113 0.1355 0.217] Comment
  (`/Game/_Core/Utils/BPC_AttackSystem.GroundSmash` (`self.BPC_Attack`) (make `/Game/_Core/Utils/S_AttackInfo` AttackTarget (`self.AnimGroundSmashAttack`) (make `/Game/_Core/Utils/S_DammageInfo` 25.0 "NewEnumerator3" "NewEnumerator1")) 300.0))

(event `BasicAttack`
  (params (AttackTarget :type "Actor Object Reference"))
  ;[0.113 0.1355 0.217] Comment
  (`/Game/_Core/Utils/BPC_AttackSystem.BasicMageSpell` (`self.BPC_Attack`) (make `/Game/_Core/Utils/S_AttackInfo` AttackTarget (`self.AnimBasicAttack`) (make `/Game/_Core/Utils/S_DammageInfo` 10.0 "NewEnumerator3"))))

(event `BarrageAttaque`
  (params (AttackTarget :type "Actor Object Reference"))
  ;[0.113 0.1355 0.217] Comment
  (`/Game/_Core/Utils/BPC_AttackSystem.BarrageMagicSpell` (`self.BPC_Attack`) (make `/Game/_Core/Utils/S_AttackInfo` AttackTarget (`self.AnimBarrage`) (make `/Game/_Core/Utils/S_DammageInfo` 15.0 "NewEnumerator2" "NewEnumerator1"))))

(event `Teleport`
  (params (Location :type "Vector Structure"))
  (bind _mesh (`self.Mesh`))
  (bind _charactermovement (`self.CharacterMovement`))
  ;[0.113 0.1355 0.217] TELEPORT START
  (if (not (`self.IsTeleporting`))
    (set `self.IsTeleporting` true)
    (`CharacterMovementComponent.SetMovementMode` _charactermovement "MOVE_Flying" 0)
    (set `CharacterMovementComponent.MaxFlySpeed` 5000.0 _charactermovement)
    (set `CharacterMovementComponent.MaxAcceleration` 99999.0 _charactermovement)
    (`SceneComponent.SetVisibility` (`self.Mesh`) false true)
    (`PrimitiveComponent.SetCollisionResponseToChannel` (`self.CapsuleComponent`) "ECC_Pawn" "ECR_Ignore")
    (bind _returnvalue (`GameplayStatics.SpawnEmitterAttached` null _mesh "spine_01"))
    (set `self.TeleportBodyEffect` _returnvalue)
    (bind _returnvalue_2 (`GameplayStatics.SpawnEmitterAttached` null _mesh "spine_01"))
    (set `self.TeleportTrailEffect` _returnvalue_2)
    (`self.StopAnimMontage` null)
    (`|AIMoveTo` self Location null
      (:`OnSuccess`
        _)
      (:`OnFail`
        _))
    (`self.TeleportEnd`)
    (else
      (`KismetSystemLibrary.DelayUntilNextTick`)
      (`self.OnTeleportEnd`))))

(event `TeleportEnd`
  (bind _charactermovement (`self.CharacterMovement`))
  ;[0.113 0.1355 0.217] TELEPORT END
  (`MovementComponent.StopMovementImmediately` _charactermovement)
  (`CharacterMovementComponent.SetMovementMode` _charactermovement "MOVE_Walking" 0)
  (set `CharacterMovementComponent.MaxAcceleration` 1500.0 _charactermovement)
  (`SceneComponent.SetVisibility` (`self.Mesh`) true true)
  (`PrimitiveComponent.SetCollisionResponseToChannel` (`self.CapsuleComponent`) "ECC_Pawn" "ECR_Block")
  (`self.OnTeleportEnd`)
  (`KismetSystemLibrary.Delay` 0.5)
  (set `self.IsTeleporting` false)
  (`|ExecutionSequence`
    (:`then_0`
      (bind _teleportbodyeffect (`self.TeleportBodyEffect`)
        (:`then`
          (`ActorComponent.K2_DestroyComponent` _teleportbodyeffect))
        (:`else`)))
    (:`then_1`
      (bind _teleporttraileffect (`self.TeleportTrailEffect`)
        (:`then`
          (`ActorComponent.K2_DestroyComponent` _teleporttraileffect))
        (:`else`)))))

(event `HealOverTime`
  (bind _returnvalue (`self.K2_GetActorLocation`))
  ;[0.113 0.1355 0.217] HEAL OVER TIME START
  (`|PlayMontage` (`self.Mesh`) (`self.AnimHeal`)
    (:`then`
      (bind (_outhit _returnvalue_2) (`KismetSystemLibrary.LineTraceSingle` _returnvalue (* _returnvalue (0.0 0.0 -1000.0)) "TraceTypeQuery1"))
      (if _returnvalue_2
        (bind _returnvalue_3 (`|SpawnActorFromClass` "/Game/_Core/AOE/BP_AOE_OverTime_Heal.BP_AOE_OverTime_Heal_C" (`KismetMathLibrary.MakeTransform` (`.Location` (`GameplayStatics.BreakHitResult` _outhit))) "Undefined" "MultiplyWithRoot" null 1.0 10.0 false false true null))
        (bind _output_get (set `self.Heal_AOE` _returnvalue_3))
        (add `/Game/_Core/AOE/BP_AOE_Base.OnAOE_OverlapActor` _output_get (delegate `OnHealTick`))
        (else
          (`self.StopAnimMontage` null))))
    (:`OnCompleted`
      (`self.HealOverTimeEnded` :!label _label))
    (:`OnInterrupted`
      (goto _label))))

(event `OnHealTick`
  (params (Actor :type "Actor Object Reference"))
  ;[0.113 0.1355 0.217] HEAL OVER TIME START
  (if (== Actor self)
    (`self.Heal` (* 0.05 (`/Game/_Core/Utils/BPC_DamageSysteme.MaxHealth` (`self.BPC_DammageSystemes`))))))

(event `HealOverTimeEnded`
  ;[0.113 0.1355 0.217] Comment
  (`self.OnHealOverTimeEnded`)
  (bind _heal_aoe (`self.Heal_AOE`)
    (:`then`
      (`self.K2_DestroyActor` _heal_aoe))
    (:`else`)))

(fn `GetIdealRange`
  (returns (AttackRadius :type "Float (double-precision)") (DefendRadius :type "Float (double-precision)"))
  (return 500.0 700.0))

(fn `SetSpeedMovement`
  (params (Speed :type "/Game/_Core/AI/Enums/E_AI_MovementSpeed Enum" :default "NewEnumerator0"))
  (returns (SpeedValue :type "Float (double-precision)"))
  (return (select `/Game/_Core/AI/Enums/E_AI_MovementSpeed` Speed :`NewEnumerator1` 125.0 :`NewEnumerator2` 250.0 :`NewEnumerator3` 400.0)))

(fn `UserConstructionScript`
  (`parent.UserConstructionScript`))