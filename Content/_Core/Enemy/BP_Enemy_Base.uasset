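; Base enemy character that fights, blocks, patrols, jumps to destinations and can be stealth-assassinated from a prompt shown near the player.
; BPC_DammageSystemes handles health and damage, with a random timed block on blockable hits.
; Its events drive hit montages and ragdoll death, switching AIC_Enemy_Base states to frozen, attacking or dead.
; Attacks reserve tokens from their target, tracked per target and returned on attack end or death.
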(event `self.ReceiveTick`
  (params (DeltaSeconds :type "Float (single-precision)"))
  ;[0.05098 0.002389 0.008662] ORIENTE WIDGET
)

(event `/Game/_Core/Utils/BPI_Dammagable.SetIsInvincible`
  (params (`IsInvincible?` :type Boolean))
  ;[0.004438 0.003772 0.05127] SET STATUS
  (set `/Game/_Core/Utils/BPC_DamageSysteme.IsInvincible?` `IsInvincible?` (`self.BPC_DammageSystemes`)))

(event `Ragdoll`
  ;[0.004438 0.003772 0.05127] ragdoll
  (`|ExecutionSequence`
    (:`then_0`
      (`KismetSystemLibrary.Delay` 2.3)
      (`PrimitiveComponent.SetSimulatePhysics` (`self.Mesh`) true))
    (:`then_1`
      (`KismetSystemLibrary.Delay` 1.5)
      (`GameplayStatics.PlaySoundAtLocation` "/Game/_Core/Sound/Hits/SQ_Death.SQ_Death" (`self.K2_GetActorLocation`) (struct) 1.0 1.0 0.0 "/Game/_Core/Sound/FootStep/SA_Character.SA_Character" null null null))))

(event `/Game/_Core/Utils/BPI_Dammagable.SetIsInterruptable`
  (params (`IsInteruptable?` :type Boolean))
  ;[0.004438 0.003772 0.05127] SET STATUS
  (set `/Game/_Core/Utils/BPC_DamageSysteme.IsInterruptible?` `IsInteruptable?` (`self.BPC_DammageSystemes`)))

(event `self.AssasineRadius.OnComponentBeginOverlap`
  (params (OverlappedComponent :type "PrimitiveComponent Object Reference") (OtherActor :type "Actor Object Reference") (OtherComp :type "PrimitiveComponent Object Reference") (OtherBodyIndex :type Integer) (bFromSweep :type Boolean) (SweepResult :type "HitResult Structure (by ref)"))
  ;[0.004438 0.003772 0.05127] affichage widget assasination on / off
  (cast `/Game/_GameMain/RPJ_Player/BP_Player` OtherActor)
  (`SceneComponent.SetVisibility` (`self.AssasinateWidget`) true false))

(event `self.ReceiveBeginPlay`
  (`|ExecutionSequence`
    (:`then_0`
      ;[0.004438 0.003772 0.05127] AIC ENEMY BASE
      (bind _asaic_enemy_base (cast `/Game/_Core/AI/AIC_Enemy_Base` (`AIBlueprintHelperLibrary.GetAIController` self)))
      (set `self.AIC_EnemyBase` _asaic_enemy_base))
    (:`then_1`
      ;[0.004438 0.003772 0.05127] SET WIDGET
      (bind _returnvalue (`|CreateWidget` "/Game/_Core/Utils/W_Enemy.W_Enemy_C" null self))
      (`WidgetComponent.SetWidget` (`self.HealthBar`) _returnvalue))
    (:`then_2`
      ;[0.05127 0.05127 0.05127] HIT REACTION
      (add `/Game/_Core/Utils/BPC_DamageSysteme.OnDammageResponse` (`self.BPC_DammageSystemes`) (`|CreateDelegate` :!event `HitResponse`)))
    (:`then_3`
      ;[0.3159 0.1019 1] RAGDOLL ENEMY DEAD COMMUN AU ENEMY BASE
      (add `/Game/_Core/Utils/BPC_DamageSysteme.OnDeath` (`self.BPC_DammageSystemes`) (`|CreateDelegate` :!event `DeathFromEB`)))))

(event `Blocked`
  (params (CanBeParried :type Boolean))
  (`KismetSystemLibrary.PrintString` "GFHDGFHDFHblock"))

(event `self.AssasineRadius.OnComponentEndOverlap`
  (params (OverlappedComponent :type "PrimitiveComponent Object Reference") (OtherActor :type "Actor Object Reference") (OtherComp :type "PrimitiveComponent Object Reference") (OtherBodyIndex :type Integer))
  ;[0.004438 0.003772 0.05127] affichage widget assasination on / off
  (cast `/Game/_GameMain/RPJ_Player/BP_Player` OtherActor)
  (`SceneComponent.SetVisibility` (`self.AssasinateWidget`) false false))

(event `HitResponse`
  (params (DamageResponse :type "/Game/_Core/Utils/E_DammageResponse Enum" :default "NewEnumerator0") (DamageCauser :type "Actor Object Reference"))
  (bind _hitreactionmontage (`self.HitReactionMontage`))
  ;[0.05127 0.05127 0.05127] HIT REACTION
  (`MovementComponent.StopMovementImmediately` (`self.CharacterMovement`))
  (`/Game/_Core/AI/AIC_Enemy_Base.SetStateAsFrozen` (`self.AIC_EnemyBase`))
  (`|PlayMontage` (`self.Mesh`) (select `/Game/_Core/Utils/E_DammageResponse` DamageResponse :`NewEnumerator0` _hitreactionmontage :`NewEnumerator1` _hitreactionmontage :`NewEnumerator2` _hitreactionmontage :`NewEnumerator3` _hitreactionmontage :`NewEnumerator4` _hitreactionmontage)
    (:`then`
      (`self.LaunchCharacter` (* (0.0 0.0 0.0) 700.0))
      (`GameplayStatics.PlaySoundAtLocation` "/Game/_Core/Sound/SoundHit/Soundhit1.Soundhit1" (`self.K2_GetActorLocation`) (struct) 1.0 (`KismetMathLibrary.RandomFloatInRange` -1.5 3.0) 0.0 "/Game/_Core/Sound/FootStep/SA_Character.SA_Character" null null null))
    (:`OnCompleted`
      (bind _teamnumber (`/Game/_Core/Utils/BPI_Dammagable.GetTeamNumber` :!label _label))
      (`/Game/_Core/AI/AIC_Enemy_Base.SetStateAsAttacking` (`self.AIC_EnemyBase`) (select `bool` (!= _teamnumber (`self.Team Number`)) :`true` DamageCauser) true))
    (:`OnInterrupted`
      (goto _label))))

(event `StartBlock`
  ;[0.004438 0.003772 0.05127] BLOCKING STATE
  (`KismetSystemLibrary.K2_ClearAndInvalidateTimerHandle` (`self.HoldBlockTimer`))
  (`KismetSystemLibrary.PrintString` "BLOCK MODE" true true (struct :`R` 0.992995 :`G` 1.0 :`B` 0.126151 :`A` 1.0) 5.0)
  (`MovementComponent.StopMovementImmediately` (`self.CharacterMovement`))
  (set `/Game/_Core/Utils/BPC_DamageSysteme.IsBlocking?` true (`self.BPC_DammageSystemes`))
  (bind _returnvalue (`KismetSystemLibrary.K2_SetTimerDelegate` (`|CreateDelegate` :!event `EndBlock`) 0.2))
  (set `self.HoldBlockTimer` _returnvalue))

(event `self.BPC_DammageSystemes.OnBlock`
  (params (CanBeParry :type Boolean) (DamageCauser :type "Actor Object Reference"))
  ;[0.004438 0.003772 0.05127] BLOCKING STATE
  (`KismetSystemLibrary.K2_ClearAndInvalidateTimerHandle` (`self.HoldBlockTimer`))
  (`|PlayMontage` (`self.Mesh`) (`self.BlockMontage`)
    (:`OnCompleted`
      _)
    (:`OnInterrupted`
      _))
  (`self.EndBlock`)
  (`self.OnBlockEnded`))

(event `EndBlock`
  ;[0.004438 0.003772 0.05127] BLOCKING STATE
  (set `/Game/_Core/Utils/BPC_DamageSysteme.IsBlocking?` false (`self.BPC_DammageSystemes`))
  (`self.OnBlockEnded`))

(event `DeathFromEB`
  (bind _reservedattacktoken (`self.ReservedAttackToken`))
  (bind _aic_enemybase (`self.AIC_EnemyBase`))
  (bind _mesh (`self.Mesh`))
  ;[0.3159 0.1019 1] RAGDOLL ENEMY DEAD COMMUN AU ENEMY BASE
  (`self.StopAnimMontage` null)
  (`PrimitiveComponent.SetSimulatePhysics` _mesh true)
  (`PrimitiveComponent.SetCollisionEnabled` _mesh "QueryAndPhysics")
  (`BrainComponent.StopLogic` (`AIController.BrainComponent` _aic_enemybase) "")
  (`/Game/_Core/AI/AIC_Enemy_Base.SetStateAsDead` _aic_enemybase)
  (`SceneComponent.SetVisibility` (`self.HealthBar`) false true)
  (bind _keys (`BlueprintMapLibrary.Map_Keys` _reservedattacktoken))
  (for _array_element _keys
    (message `/Game/_Core/Utils/BPI_Dammagable.ReturnAttackToken` _array_element (`BlueprintMapLibrary.Map_Find` _reservedattacktoken _array_element))))

(event `/Game/_Core/AI/BPI_Enemy_Base_AI.JumpToDestination`
  (params (Destination :type "Vector Structure"))
  ;[0.004438 0.003772 0.05127] Jump to destination
  (bind _outlaunchvelocity (`GameplayStatics.SuggestProjectileVelocity_CustomArc` (`self.K2_GetActorLocation`) (`KismetMathLibrary.MakeVector` (.x Destination) (.y Destination) (+ (.z Destination) 250.0))))
  (`self.LaunchCharacter` _outlaunchvelocity true true))

(event `/Game/_Core/Utils/BPI_Dammagable.ReturnAttackToken`
  (params (Integer :type Integer))
  ;[0.004438 0.003772 0.05127] GESTION TOKEN
  (`/Game/_Core/Utils/BPC_DamageSysteme.ReturnAttackToken` (`self.BPC_DammageSystemes`) Integer))

(event `/Game/_Core/AI/BPI_Enemy_Base_AI.StoreAttackToken`
  (params (AttackTarget :type "Actor Object Reference") (Amount :type Integer))
  (bind (_value _returnvalue) (`BlueprintMapLibrary.Map_Find` (`self.ReservedAttackToken`) AttackTarget))
  ;[0.004438 0.003772 0.05127] GESTION TOKEN
  (`BlueprintMapLibrary.Map_Add` (`self.ReservedAttackToken`) AttackTarget (`KismetMathLibrary.SelectInt` (+ Amount _value) Amount _returnvalue)))

(event `/Game/_Core/AI/BPI_Enemy_Base_AI.Attack`
  (params (AttackTarget :type "Actor Object Reference"))
  ;[0.004438 0.003772 0.05127] GESTION TOKEN
  (set `self.isAttacking?` true))

(event `/Game/_Core/AI/BPI_Enemy_Base_AI.AttackEnd`
  (params (AttackTarget :type "Actor Object Reference"))
  (bind _tokenusedincurrentattack (`self.TokenUsedInCurrentAttack`))
  ;[0.004438 0.003772 0.05127] GESTION TOKEN
  (message `/Game/_Core/Utils/BPI_Dammagable.ReturnAttackToken` AttackTarget _tokenusedincurrentattack)
  (`/Game/_Core/AI/BPI_Enemy_Base_AI.StoreAttackToken` AttackTarget (* _tokenusedincurrentattack -1))
  (set `self.isAttacking?` false)
  (`self.OnAttackEnd`))

(fn `AttackStart`
  (params (AttackTarget :type "Actor Object Reference") (TokenNeeded :type Integer))
  (returns (Succes :type Boolean))
  (bind _succes (message `/Game/_Core/Utils/BPI_Dammagable.ReserveAttackToken` AttackTarget TokenNeeded))
  (if _succes
    (`/Game/_Core/AI/BPI_Enemy_Base_AI.StoreAttackToken` AttackTarget TokenNeeded)
    (set `self.TokenUsedInCurrentAttack` TokenNeeded)
    (return true)
    (else
      (return false))))

(fn `GetCurrentHealth`
  (returns (CurrentHealth :type "Float (double-precision)"))
  (return (`/Game/_Core/Utils/BPC_DamageSysteme.CurrentHealth` (`self.BPC_DammageSystemes`))))

(fn `GetCurrentLevel`
  (returns (CurrentLevel :type Integer))
  (return 0))

(fn `GetCurrentMana`
  (returns (CurrentMana :type "Float (double-precision)"))
  (return 0.0))

(fn `GetCurrentStamina`
  (returns (CurrentStamina :type "Float (double-precision)"))
  (return 0.0))

(fn `GetCurrentXP`
  (returns (CurrentXP :type "Float (double-precision)"))
  (return 0.0))

(fn `GetIdealRange`
  (returns (AttackRadius :type "Float (double-precision)") (DefendRadius :type "Float (double-precision)"))
  (return 150.0 350.0))

(fn `GetMaxHealth`
  (returns (MaxHealth :type "Float (double-precision)"))
  (return (`/Game/_Core/Utils/BPC_DamageSysteme.MaxHealth` (`self.BPC_DammageSystemes`))))

(fn `GetMaxMana`
  (returns (MaxLevel :type "Float (double-precision)"))
  (return 0.0))

(fn `GetMaxStamina`
  (returns (MaxStamina :type "Float (double-precision)"))
  (return 0.0))

(fn `GetMaxXP`
  (returns (MaxXP :type "Float (double-precision)"))
  (return 0.0))

(fn `GetPatrolRoute`
  (returns (PatrolRoute :type "/Game/_Core/AI/BP_PatrolRoute Object Reference"))
  (return (`self.PatrolRoute`)))

(fn `GetTeamNumber`
  (returns (TeamNumber :type Integer))
  (return (`self.Team Number`)))

(fn `Heal`
  (params (Amount :type "Float (double-precision)"))
  (returns (NewHealth :type "Float (double-precision)"))
  (bind _newhealth (`/Game/_Core/Utils/BPC_DamageSysteme.Heal` (`self.BPC_DammageSystemes`) Amount))
  (return _newhealth))

(fn `IsAttacking`
  (returns (`IsAttacking?` :type Boolean))
  (return false))

(fn `IsDead`
  (returns (`IsDead?` :type Boolean))
  (return (`/Game/_Core/Utils/BPC_DamageSysteme.IsDead?` (`self.BPC_DammageSystemes`))))

(fn `ReserveAttackToken`
  (params (Amount :type Integer))
  (returns (Succes :type Boolean))
  (bind _succes (`/Game/_Core/Utils/BPC_DamageSysteme.ReserveAttackToken` (`self.BPC_DammageSystemes`) Amount))
  (return _succes))

(fn `SetMovementSpeed`
  (params (Speed :type "/Game/_Core/AI/Enums/E_AI_MovementSpeed Enum" :default "NewEnumerator0"))
  (returns (SpeedValue :type "Float (double-precision)"))
  (set `CharacterMovementComponent.MaxWalkSpeed` (select `/Game/_Core/AI/Enums/E_AI_MovementSpeed` Speed :`NewEnumerator1` 100.0 :`NewEnumerator2` 200.0 :`NewEnumerator3` 300.0 :!type "Float (single-precision)") (`self.CharacterMovement`))
  (return 0.0))

(fn `SetSpeedMovement`
  (params (Speed :type "/Game/_Core/AI/Enums/E_AI_MovementSpeed Enum" :default "NewEnumerator0"))
  (returns (SpeedValue :type "Float (double-precision)"))
  (bind _output_get (set `CharacterMovementComponent.MaxWalkSpeed` (select `/Game/_Core/AI/Enums/E_AI_MovementSpeed` Speed :`NewEnumerator1` 100.0 :`NewEnumerator2` 300.0 :`NewEnumerator3` 500.0) (`self.CharacterMovement`)))
  (return _output_get))

(fn `StealthBackAssasin`
  (returns (RefLocation :type "Vector Structure") (RefRotation :type "Rotator Structure"))
  (`self.PlayAnimMontage` "/Game/_GameMain/RPJ_Enemy/Animation/Paired_Knife_Stealth_KidneyAndNeck_Vic_Montage.Paired_Knife_Stealth_KidneyAndNeck_Vic_Montage")
  (`self.Ragdoll`)
  (`SceneComponent.SetVisibility` (`self.AssasinateWidget`) false false)
  (return (`SceneComponent.K2_GetComponentLocation` (`self.AssasineRef`)) (`self.K2_GetActorRotation`)))

(fn `TakeDamage`
  (params (DamageInfo :type "/Game/_Core/Utils/S_DammageInfo Structure") (DamageCauser :type "Actor Object Reference"))
  (returns (WasDamage :type Boolean))
  (if (`.CanBeBlock_19_9864068D4C58D2972DC243AA057931DE` (break `/Game/_Core/Utils/S_DammageInfo` DamageInfo))
    (`self.TryToBlock`))
  (bind _wasdamaged (`/Game/_Core/Utils/BPC_DamageSysteme.TakeDamage` (`self.BPC_DammageSystemes`) DamageInfo DamageCauser))
  (return _wasdamaged))

(fn `TryToBlock`
  (if (<= (`KismetMathLibrary.RandomFloat`) (`self.BlockChance`))
    (`self.StartBlock`)))

(fn `UserConstructionScript`)