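; Boss enemy Blueprint extending a parent enemy, with its own health and a health bar widget updated on damage.
; Attack events combine BPCAttack calls with montage notifies for melee combos, smash, jump, homing axe and lightning AOE.
; Teleport is faked by hiding the mesh and flying rapidly via AIMoveTo, signalling completion by dispatcher.
; Floating spawns a platform and grants invincibility; weapon equip/unequip and the platform's StopFloating call are disconnected.
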(event `self.ReceiveBeginPlay`
  (bind _bpc_dammagesystemes (`self.BPC_DammageSystemes`))
  ;[0.113 0.1355 0.217] health bar
  (`parent.ReceiveBeginPlay`)
  (`WidgetComponent.SetWidget` (`self.HealthBar`) null)
  (bind _returnvalue (`|CreateWidget` "/Game/_Core/Utils/W_BossHelthBar.W_BossHelthBar_C"))
  (bind _output_get (set `self.BossHealthbarWidgetRef` _returnvalue))
  (`/Game/_Core/Utils/W_BossHelthBar.UpdateHealthPourcentage` _output_get (`/Game/_Core/Utils/BPC_DamageSysteme.CurrentHealth` _bpc_dammagesystemes) (`/Game/_Core/Utils/BPC_DamageSysteme.MaxHealth` _bpc_dammagesystemes)))

(event `Teleport`
  (params (Location :type "Vector Structure") (AttackTarget :type "Actor Object Reference"))
  (bind _mesh (`self.Mesh`))
  (bind _charactermovement (`self.CharacterMovement`))
  ;[0.1684 0.135 0.1412] TELEPORT START
  (if (not (`self.IsTeleporting`))
    (set `self.IsTeleporting` true)
    (`CharacterMovementComponent.SetMovementMode` _charactermovement "MOVE_Flying" 0)
    (set `CharacterMovementComponent.MaxFlySpeed` 5000.0 _charactermovement)
    (set `CharacterMovementComponent.MaxAcceleration` 99999.0 _charactermovement)
    (`SceneComponent.SetVisibility` (`self.Mesh`) false true)
    (`PrimitiveComponent.SetCollisionResponseToChannel` (`self.CapsuleComponent`) "ECC_Pawn" "ECR_Ignore")
    ;;[1 0 0] retiré
    (bind _returnvalue (`GameplayStatics.SpawnEmitterAttached` null _mesh "Spine1"))
    (set `self.TeleportBodyEffect` _returnvalue)
    (bind _returnvalue_2 (`GameplayStatics.SpawnEmitterAttached` null _mesh "Spine1"))
    (set `self.TeleportTrailEffect` _returnvalue_2)
    (`self.StopAnimMontage` null)
    (`|AIMoveTo` self Location AttackTarget 150.0
      (:`OnSuccess`
        _)
      (:`OnFail`
        _))
    (`self.TeleportEnd`)
    (else
      (`KismetSystemLibrary.DelayUntilNextTick`)
      (`self.OnTeleportEnd`))))

(event `/Game/_Core/AI/BPI_Enemy_Base_AI.EquipWeapon`)

(event `TeleportEnd`
  (bind _charactermovement (`self.CharacterMovement`))
  ;[0.1684 0.135 0.1412] TELEPORT END
  (`MovementComponent.StopMovementImmediately` _charactermovement)
  (`CharacterMovementComponent.SetMovementMode` _charactermovement "MOVE_Walking" 0)
  (set `CharacterMovementComponent.MaxAcceleration` 1500.0 _charactermovement)
  (`SceneComponent.SetVisibility` (`self.Mesh`) true true)
  (`PrimitiveComponent.SetCollisionResponseToChannel` (`self.CapsuleComponent`) "ECC_Pawn" "ECR_Block")
  (`self.OnTeleportEnd`)
  (`KismetSystemLibrary.Delay` 0.5)
  (set `self.IsTeleporting` false)
  (`|ExecutionSequence`
    (:`then_0`
      ;;[1 0.008681 0.008681] retire
      (bind _teleportbodyeffect (`self.TeleportBodyEffect`)
        (:`then`
          (`ActorComponent.K2_DestroyComponent` _teleportbodyeffect))
        (:`else`)))
    (:`then_1`
      (bind _teleporttraileffect (`self.TeleportTrailEffect`)
        (:`then`
          (`ActorComponent.K2_DestroyComponent` _teleporttraileffect))
        (:`else`)))))

(event `/Game/_Core/AI/BPI_Enemy_Base_AI.UnequipWeapon`)

(event `AttackCombo1`
  (params (AttackTarget :type "Actor Object Reference"))
  ;[0.08592 0.217 0.1902] attack  combo 1
  (`/Game/_Core/Utils/BPC_AttackSystem.PrimaryMeleAttaque` (`self.BPC_Attack`) (make `/Game/_Core/Utils/S_AttackInfo` null (`self.MontageCombo1`) (make `/Game/_Core/Utils/S_DammageInfo` 20.0 "NewEnumerator1" "NewEnumerator1" false true true)) 40.0 250.0))

(event `StartFloat`
  (bind _returnvalue (`self.K2_GetActorLocation`))
  ;[0.224 0.04705 0.1572] PLATEFORMSTARTFLOATING
  (set `/Game/_Core/Utils/BPC_DamageSysteme.IsInvincible?` true (`self.BPC_DammageSystemes`))
  (bind _outhit (`KismetSystemLibrary.LineTraceSingle` _returnvalue (* _returnvalue (0.0 0.0 -1000.0)) "TraceTypeQuery1"))
  (bind _returnvalue_2 (`|SpawnActorFromClass` "/Game/_Core/Props/BP_FloatingPlateform.BP_FloatingPlateform_C" (`KismetMathLibrary.MakeTransform` (`.Location` (`GameplayStatics.BreakHitResult` _outhit))) "Undefined" "MultiplyWithRoot" null null))
  (bind _output_get (set `self.FloatingPlateformeRef` _returnvalue_2))
  (add `/Game/_Core/Props/BP_FloatingPlateform.OnFloatTimelineFinished` _output_get (delegate `OnFloorTimelineFinished_Event`)))

(event `OnFloorTimelineFinished_Event`
  ;[0.224 0.04705 0.1572] PLATEFORMSTARTFLOATING
  (remove `/Game/_Core/Props/BP_FloatingPlateform.OnFloatTimelineFinished` (stale `StartFloat` _output_get) (delegate `OnFloorTimelineFinished_Event`))
  (`self.OnFloatHeightReached`))

(event `StopFloat`
  ;[0.224 0.04705 0.1572] PLATEFORMSTARTFLOATING
  (bind _floatingplateformeref (`self.FloatingPlateformeRef`)
    (:`then`
      (`self.StopFloat`))
    (:`else`
      (`KismetSystemLibrary.DelayUntilNextTick`)
      (set `/Game/_Core/Utils/BPC_DamageSysteme.IsInvincible?` false (`self.BPC_DammageSystemes`) :!label _label)
      (`self.OnFloatEnded`))))

(event `AttackCombo2`
  (params (AttackTarget :type "Actor Object Reference"))
  (bind _bpc_attack (`self.BPC_Attack`))
  ;[0.08592 0.217 0.1902] attack combo 2
  (`self.Attack` AttackTarget)
  (bind _notifyname (`|PlayMontage` (`self.Mesh`) (`self.MontageCombo2`))
    (:`OnCompleted`
      (`self.AttackEnd` AttackTarget :!label _label_2))
    (:`OnInterrupted`
      (goto _label_2))
    (:`OnNotifyBegin`
      (switch `name` _notifyname
        (:`Slash`
          (`/Game/_Core/Utils/BPC_AttackSystem.SphereTraceDamage` _bpc_attack (make `/Game/_Core/Utils/S_DammageInfo` 15.0 "NewEnumerator1" "NewEnumerator1" false true true) 40.0 200.0))
        (:`AOESlash`
          (`/Game/_Core/Utils/BPC_AttackSystem.AOEDamage` _bpc_attack 300.0 (make `/Game/_Core/Utils/S_DammageInfo` 20.0 "NewEnumerator3" "NewEnumerator1" false false false true)))))))

(event `OnFloatTimelineFinished`
  ;[0.224 0.04705 0.1572] PLATEFORMSTARTFLOATING
  (remove `/Game/_Core/Props/BP_FloatingPlateform.OnFloatTimelineFinished` (stale `StopFloat` _floatingplateformeref) (delegate `OnFloatTimelineFinished`))
  (`self.K2_DestroyActor` (stale `StopFloat` _floatingplateformeref))
  (goto _label))

(event `OnFloatTimelineFinshed_Event`
  ;[0.224 0.04705 0.1572] PLATEFORMSTARTFLOATING
)

(event `Throw axe`
  (params (AttackTarget :type "Actor Object Reference"))
  ;[0.08592 0.217 0.1902] THROW AXE
  (`self.Attack` AttackTarget)
  (bind _notifyname (`|PlayMontage` (`self.Mesh`))
    (:`OnCompleted`
      (`SceneComponent.SetVisibility` (`/Game/_Core/Weapon/MeleWeapon/BP_Weapon_Base.WeaponSKM` (`self.WeaponActor`)) true false :!label _label_3)
      (`/Game/_Core/AI/BPI_Enemy_Base_AI.AttackEnd` AttackTarget))
    (:`OnInterrupted`
      (goto _label_3))
    (:`OnNotifyBegin`
      (switch `name` _notifyname
        (:`Throw`
          (`SceneComponent.SetVisibility` (`/Game/_Core/Weapon/MeleWeapon/BP_Weapon_Base.WeaponSKM` (`self.WeaponActor`)) false false)
          (bind _returnvalue (`|SpawnActorFromClass` "/Game/_Core/Weapon/MagicWeapon/BP_Projectile_SpinningAxe.BP_Projectile_SpinningAxe_C" (`KismetMathLibrary.MakeTransform` (`SceneComponent.GetSocketLocation` (`self.Mesh`) "RightWeapon")) "Undefined" "MultiplyWithRoot" null 4000.0 0.0 AttackTarget true (1.0 1.0 1.0) self))
          (add `/Game/_Core/Weapon/MagicWeapon/BP_Projectile_Base.OnProjectileImpact` _returnvalue (delegate `OnProjectileImpact_Event`)))))))

(event `OnProjectileImpact_Event`
  (params (OtherActor :type "Actor Object Reference") (HitResult :type "HitResult Structure"))
  ;[0.08592 0.217 0.1902] THROW AXE
  (message `/Game/_Core/Utils/BPI_Dammagable.TakeDamage` OtherActor (make `/Game/_Core/Utils/S_DammageInfo` 20.0 "NewEnumerator2" "NewEnumerator1" false true) self))

(event `QuickAttack`
  (params (AttackTarget :type "Actor Object Reference"))
  ;[0.08592 0.217 0.1902] QUICK ATTACK
  (`/Game/_Core/Utils/BPC_AttackSystem.PrimaryMeleAttaque` (`self.BPC_Attack`) (make `/Game/_Core/Utils/S_AttackInfo` AttackTarget null (make `/Game/_Core/Utils/S_DammageInfo` 20.0 "NewEnumerator1" "NewEnumerator1" false true true)) 40.0 250.0))

(event `GroundSmash`
  (params (AttackTarget :type "Actor Object Reference"))
  ;[0.08592 0.217 0.1902] Ground smash
  (`/Game/_Core/Utils/BPC_AttackSystem.GroundSmash` (`self.BPC_Attack`) (make `/Game/_Core/Utils/S_AttackInfo` AttackTarget (`self.MontageGroundAttack`) (make `/Game/_Core/Utils/S_DammageInfo` 25.0 "NewEnumerator3" "NewEnumerator1" false false false true)) 1100.0))

(event `JumpAttack`
  (params (AttackTarget :type "Actor Object Reference"))
  ;[0.08592 0.217 0.1902] JUMP ATTACK
  (`/Game/_Core/Utils/BPC_AttackSystem.LongRangeMeleAttack` (`self.BPC_Attack`) (make `/Game/_Core/Utils/S_AttackInfo` AttackTarget null (make `/Game/_Core/Utils/S_DammageInfo` 20.0 "NewEnumerator3" "NewEnumerator1" false false false true))))

(event `AOETrail`
  (params (AttackTarget :type "Actor Object Reference"))
  ;[1 1 1] Comment
  (`self.Attack` AttackTarget)
  (bind _notifyname (`|PlayMontage` (`self.Mesh`))
    (:`OnCompleted`
      (`self.AttackEnd` AttackTarget :!label _label_4))
    (:`OnInterrupted`
      (goto _label_4))
    (:`OnNotifyBegin`
      (switch `name` _notifyname
        (:`Strike`
          (bind _returnvalue (`|SpawnActorFromClass` "/Game/_Core/AOE/BP_AOE_Blast_Lightning.BP_AOE_Blast_Lightning_C" (`KismetMathLibrary.MakeTransform` (0.0 0.0 0.0)) "Undefined" "MultiplyWithRoot" null 3.0 AttackTarget null false true false null))
          (add `/Game/_Core/AOE/BP_AOE_Base.OnAOE_OverlapActor` _returnvalue (delegate `OnAOEOverlapActor_Event`)))))))

(event `OnAOEOverlapActor_Event`
  (params (Actor :type "Actor Object Reference"))
  ;[1 1 1] Comment
  (bind _teamnumber (message `/Game/_Core/Utils/BPI_Dammagable.GetTeamNumber` Actor))
  (if (!= _teamnumber (`self.Team Number`))
    (message `/Game/_Core/Utils/BPI_Dammagable.TakeDamage` Actor (make `/Game/_Core/Utils/S_DammageInfo` 5.0 "NewEnumerator3" "NewEnumerator1") self)))

(fn `SetSpeedMovement`
  (params (Speed :type "/Game/_Core/AI/Enums/E_AI_MovementSpeed Enum" :default "NewEnumerator0"))
  (returns (SpeedValue :type "Float (double-precision)"))
  (set `CharacterMovementComponent.MaxWalkSpeed` (select `/Game/_Core/AI/Enums/E_AI_MovementSpeed` Speed :`NewEnumerator1` 100.0 :`NewEnumerator2` 200.0 :`NewEnumerator3` 350.0 :!type "Float (single-precision)") (`self.CharacterMovement`))
  (return 0.0))

(fn `TakeDamage`
  (params (DamageInfo :type "/Game/_Core/Utils/S_DammageInfo Structure") (DamageCauser :type "Actor Object Reference"))
  (returns (WasDamage :type Boolean))
  (bind _bpc_dammagesystemes (`self.BPC_DammageSystemes`))
  (bind _wasdamage (`parent.TakeDamage` DamageInfo DamageCauser))
  (`/Game/_Core/Utils/W_BossHelthBar.UpdateHealthPourcentage` (`self.BossHealthbarWidgetRef`) (`/Game/_Core/Utils/BPC_DamageSysteme.CurrentHealth` _bpc_dammagesystemes) (`/Game/_Core/Utils/BPC_DamageSysteme.MaxHealth` _bpc_dammagesystemes))
  (return _wasdamage))

(fn `UserConstructionScript`
  (bind _bpc_dammagesystemes (`self.BPC_DammageSystemes`))
  (`parent.UserConstructionScript`)
  (set `/Game/_Core/Utils/BPC_DamageSysteme.MaxHealth` 700.0 _bpc_dammagesystemes)
  (set `/Game/_Core/Utils/BPC_DamageSysteme.CurrentHealth` 700.0 _bpc_dammagesystemes))