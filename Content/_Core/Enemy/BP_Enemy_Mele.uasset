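; Melee enemy character that wields a sword, built on a parent enemy Blueprint.
; Equip and unequip montages use notifies to spawn and socket-attach or destroy the sword, and report completion.
; Short-range, long-range, spinning and ground-smash attacks pass montage and damage info to BPCAttack, while GetIdealRange supplies attack and defend radii.
; Older trace, predicted-leap, AOE and blocking logic remains as legacy helpers or unconnected graphs.
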(event Custom|StopSpinning
  ;[0.03299 0.003722 0.003722] TO DELETE
  ;;[1 0.9456 0.05527] Comment
  (Audio|Components|Audio|Stop (Variables|Default|GetSpinMeshTimeline))
  (Transformation|SetRelativeRotation (Variables|Character|GetMesh) (Variables|Default|GetMeshRotationBeforeSpin) false false))

(event Custom|AOESlash%28Old%29
  (params (AttackTarget :type Actor%20Object%20Reference))
  ;[0.03299 0.003722 0.003722] TO DELETE
  ;;[0.3159 0.1019 1] ATTACK HELPER
  ;;;[1 0.005208 0.005208] Comment
  (bind _returnvalue (Game|SpawnActorfromClass "/Game/_Core/AOE/BP_AOE_Base.BP_AOE_Base_C" (Math|Transform|MakeTransform (Transformation|GetActorLocation) "0, 0, 0" "1.000000,1.000000,1.000000") "Undefined" "MultiplyWithRoot" 0 true true false self))
  (Variables|/Game/_Core/AOE/BP_AOE_Base.BP_AOE_Base_C|SetRadius _returnvalue 3e+02)
  (EventDispatchers|BindEventtoOnAOEOverlapActor _returnvalue (delegate Custom|DamageActorOnEOEActor))
  (Default|Trigger _returnvalue))

(event Custom|DamageActorOnEOEActor
  (params (Actor :type Actor%20Object%20Reference))
  ;[0.03299 0.003722 0.003722] TO DELETE
  ;;[0.3159 0.1019 1] ATTACK HELPER
  ;;;[1 0.005208 0.005208] Comment
  (if (== Actor (stale Custom|AOESlash%28Old%29 AttackTarget))
    (Class|BPIDammagable|TakeDamage(Message) Actor (Utilities|Struct|MakeS_DammageInfo 1e+01 "NewEnumerator1" "NewEnumerator1" false true) self)))

(event Custom|SpinMesh
  ;[0.03299 0.003722 0.003722] TO DELETE
  ;;[1 0.9456 0.05527] Comment
  (Variables|Default|SetMeshRotationBeforeSpin (Variables|/Script/Engine.SceneComponent|GetRelativeRotation (Variables|Character|GetMesh)))
  (bind _zrotationalpha (Timeline|SpinMeshTimeline PlayFromStart)
    (:Update
      (Transformation|SetRelativeRotation (Variables|Character|GetMesh) (Math|Rotator|MakeRotator (.roll (Variables|Default|GetMeshRotationBeforeSpin)) (.pitch (Variables|Default|GetMeshRotationBeforeSpin)) (Math|Float|Lerp (.yaw (Variables|Default|GetMeshRotationBeforeSpin)) (+ (.yaw (Variables|Default|GetMeshRotationBeforeSpin)) (|(360*5))) _zrotationalpha)) false false))))

(event Custom|ShortRangeAttack
  (params (AttackTarget :type Actor%20Object%20Reference))
  ;[0.113 0.1355 0.217] ATTAQUE
  (Default|PrimaryMeleAttaque (Variables|Default|GetBPC_Attack) (Utilities|Struct|MakeS_AttackInfo AttackTarget (Variables|Attack|GetAttack_ShortRange) (Utilities|Struct|MakeS_DammageInfo 1e+01 "NewEnumerator1" "NewEnumerator1" false true true)) 2e+01 2e+02))

(event Custom|LongRangeAttack
  (params (AttackTarget :type Actor%20Object%20Reference))
  ;[0.113 0.1355 0.217] ATTAQUE
  (Default|LongRangeMeleAttack (Variables|Default|GetBPC_Attack) (Utilities|Struct|MakeS_AttackInfo AttackTarget (Variables|Attack|GetAttack_LongRange) (Utilities|Struct|MakeS_DammageInfo 2e+01 "NewEnumerator1" "NewEnumerator0" false false true))))

(event Custom|SphereTraceDamage%28OLD%29
  (bind _returnvalue (Transformation|GetActorLocation))
  ;[0.03299 0.003722 0.003722] TO DELETE
  ;;[0.3159 0.1019 1] ATTACK HELPER
  ;;;[1 0.005208 0.005208] Comment
  (Development|PrintString "ON FAIT DU DOMMAGE" true true "(R=0.315919,G=0.101902,B=1.000000,A=1.000000)" 5.0)
  (bind (_outhits _returnvalue_2) (Collision|MultiSphereTraceForObjects _returnvalue (+ _returnvalue (* (Transformation|GetActorForwardVector) 2e+02)) 2e+01 (Utilities|Array|MakeArray "ObjectTypeQuery3") false 0 "None"))
  (if _returnvalue_2
    (Default|DammageAllNonTeamMember (Variables|Default|GetBPC_Attack) _outhits (Utilities|Struct|MakeS_DammageInfo 1e+01 "NewEnumerator1"))))

(event Custom|JumpToAttackTarget%28OLD%29
  (params (ActorTarget :type Actor%20Object%20Reference))
  ;[0.03299 0.003722 0.003722] TO DELETE
  ;;[0.3159 0.1019 1] ATTACK HELPER
  ;;;[1 0 0] Comment
  (bind _location (CallFunction|CalculateFutureActorLocation ActorTarget 1.0))
  (bind _outlaunchvelocity (Game|SuggestProjectileVelocityCustomArc (Transformation|GetActorLocation) (Math|Vector|MakeVector (.x _location) (.y _location) (+ (.z _location) 1e+02)) 0.0 0.5))
  (Character|LaunchCharacter _outlaunchvelocity true true)
  (EventDispatchers|BindEventtoLandedDelegate (delegate Custom|AttEnd)))

(event Custom|AttEnd
  (params (Hit :type Hit%20Result%20Structure%20%28by%20ref%29))
  ;[0.03299 0.003722 0.003722] TO DELETE
  ;;[0.3159 0.1019 1] ATTACK HELPER
  ;;;[1 0 0] Comment
  (EventDispatchers|UnbindEventfromLandedDelegate (delegate Custom|AttEnd))
  (Components|Movement|StopMovementImmediately (Variables|Character|GetCharacterMovement)))

(event Custom|SpinningAttack
  (params (AttackTarget :type Actor%20Object%20Reference))
  ;[0.113 0.1355 0.217] ATTAQUE
  (Default|SpinningMeleAttack (Variables|Default|GetBPC_Attack) (Utilities|Struct|MakeS_AttackInfo AttackTarget (Variables|Attack|GetAttack_Spinning) (Utilities|Struct|MakeS_DammageInfo 1e+01 "NewEnumerator1" "NewEnumerator1" false true))))

(event Custom|GroundSmashAttack
  (params (AttackTarget :type Actor%20Object%20Reference))
  ;[0.113 0.1355 0.217] ATTAQUE
  (Default|GroundSmash (Variables|Default|GetBPC_Attack) (Utilities|Struct|MakeS_AttackInfo 0 (Variables|Attack|GetAttack_GroundSmash) (Utilities|Struct|MakeS_DammageInfo 25.0 "NewEnumerator1" "NewEnumerator1")) 3e+02))

(event Custom|ChaseAttackTarget
  (params (AttackTarget :type Actor%20Object%20Reference))
  ;[0.03299 0.003722 0.003722] TO DELETE
  ;;[1 0.9456 0.05527] Comment
  (AI|AIMoveTo self "0, 0, 0" AttackTarget 5.0 false
    (:OnSuccess
      (Utilities|FlowControl|Delay 0.1)
      (if (Variables|Default|GetisAttacking?)
        (CallFunction|ChaseAttackTarget AttackTarget)))))

(event EventUnEquipWeapon
  ;[0.05374 1 0.1893] On joue le montage de ranger l'épee et on set la variable is wielding weapon a FALSE
  (bind _notifyname (Animation|Montage|PlayMontage (Variables|Character|GetMesh) 0)
    (:OnCompleted
      (Default|CallOnWeaponUnequip))
    (:OnNotifyBegin
      (switch name _notifyname
        (:DropSword
          (Actor|DestroyActor (Variables|Default|GetWeaponActor))
          (Variables|Default|SetisWieldingWeapon false))))))

(event EventEquipWeapon
  ;[0.05374 1 0.1893] On joue le montage de sortir l'épée set la variable is wielding weapon a TRUE
  (bind _notifyname (Animation|Montage|PlayMontage (Variables|Character|GetMesh) 0)
    (:OnCompleted
      (Default|CallOnWeaponEquip))
    (:OnNotifyBegin
      (switch name _notifyname
        (:HoldSword
          (bind _returnvalue (Game|SpawnActorfromClass :Class "/Game/_Core/Weapon/MeleWeapon/BP_Weapon_Sword.BP_Weapon_Sword_C" :SpawnTransform (Transformation|GetActorTransform) :CollisionHandlingOverride "Undefined" :TransformScaleMethod "MultiplyWithRoot" :Instigator 0))
          (bind _output_get (Variables|Default|SetWeaponActor _returnvalue))
          (Transformation|AttachComponentToComponent _output_get (Variables|Character|GetMesh) "Hand_R_Sword_Socket" "SnapToTarget" "SnapToTarget" "SnapToTarget" true)
          (Variables|Default|SetisWieldingWeapon true))))))

(event EventTick
  (params (DeltaSeconds :type Float%20%28single-precision%29)))

(event EventBeginPlay
  ;[0.113 0.1355 0.217] INIT PLAYER
  (|CallParentFunction)
  (CallFunction|SetSpeedMovement "NewEnumerator1"))

(event Collision|EventActorBeginOverlap
  (params (OtherActor :type Actor%20Object%20Reference)))

(fn ConstructionScript
  (|CallParentFunction)
  (Variables|Default|SetMeshRotationBeforeSpin (Variables|/Script/Engine.SceneComponent|GetRelativeRotation (Variables|Character|GetMesh))))

(fn GetIdealRange
  (return 2e+02 4e+02))

(fn CalculateFutureActorLocation
  (params (Actor :type Actor%20Object%20Reference) (Time :type Float%20%28double-precision%29))
  ;[1 1 1] Location est la velocite x current location
  (return (+ (Transformation|GetActorLocation Actor) (* (* (Transformation|GetVelocity Actor) "1.000000,1.000000,0.000000") Time))))