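; BP_PatrolRoute is an AI patrol route that defines its waypoints as the points of a PatrolRoute spline.
; IncrementPatrolRoute steps PatrolIndex by Direction and flips Direction at either end of the spline, so traversal ping-pongs back and forth.
; GetSplinePointAtWorldPosition returns the world location of the spline point at the current index.
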(event `IncrementPatrolRoute`
  ;[0.03098 0.8232 1] Incremente l'index des points sur la patrol route en fonction direction 1 ou -1
  (bind _output_get (set `self.PatrolIndex` (+ (`self.PatrolIndex`) (`self.Direction`))))
  ;[0.03098 0.8232 1] Verifie si on arrive a un des bouts de la spline
  (if (== _output_get (- (`SplineComponent.GetNumberOfSplinePoints` (`self.PatrolRoute`)) 1))
    (set `self.Direction` -1)
    (elif (== (`self.PatrolIndex`) 0)
      (set `self.Direction` 1))))

(fn `GetSpline Point AtWorldPosition`
  (returns (Location :type "Vector Structure"))
  (return (`SplineComponent.GetLocationAtSplinePoint` (`self.PatrolRoute`) (`self.PatrolIndex`) "World")))

(fn `UserConstructionScript`)