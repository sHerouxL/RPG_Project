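; Attack component that gives its owning character melee, bullet, spell, lightning, AOE and healing attacks.
; Most attacks play montages whose notifies trigger traces, spawned projectiles or AOE actors, plus a leap arced toward the target's predicted position.
; Damage and attack state go to actors through interface messages, with team filtering on most melee, bullet and AOE hits.
; A separate simple combo steps through a montage list, using notifies to box-trace damage and reset.
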(event `MagicSpell`
  (params (SpawnTransform :type "Transform Structure") (Target :type "Actor Object Reference") (DamageInfo :type "/Game/_Core/Utils/S_DammageInfo Structure") (Alt :type Boolean))
  ;[0.008875 0.05971 0.3802] Magic spell attack
  (`KismetSystemLibrary.PrintString` "Magic spell")
  (bind _returnvalue (`|SpawnActorFromClass` (select `bool` Alt :`false` "/Game/_Core/Weapon/MagicWeapon/CBP_BlackBall.CBP_BlackBall_C" :`true` "/Game/_Core/Weapon/MagicWeapon/CBP_MageBarrage.CBP_MageBarrage_C" :!type "/Game/_Core/Weapon/MagicWeapon/BP_Projectile_Base Class Reference") SpawnTransform "Undefined" "MultiplyWithRoot" (`self.GetOwner`) 1000.0 0.0 Target false (1.0 1.0 1.0) null))
  (add `/Game/_Core/Weapon/MagicWeapon/BP_Projectile_Base.OnProjectileImpact` _returnvalue (delegate `OnProjectileHit`))
  (`PrimitiveComponent.IgnoreActorWhenMoving` (`Actor.GetComponentByClass` (`self.GetOwner`) "/Script/Engine.CapsuleComponent") _returnvalue true))

(event `OnProjectileHit`
  (params (OtherActor :type "Actor Object Reference") (HitResult :type "HitResult Structure"))
  (bind _returnvalue (`self.GetOwner`))
  ;[0.008875 0.05971 0.3802] Magic spell attack
  (message `/Game/_Core/Utils/BPI_Dammagable.TakeDamage` OtherActor (stale `MagicSpell` DamageInfo) _returnvalue)
  (`AISense_Damage.ReportDamageEvent` OtherActor _returnvalue (`.Amount_2_372379F2408E17C0DE5E86A6585F6FE9` (break `/Game/_Core/Utils/S_DammageInfo` (stale `MagicSpell` DamageInfo))) (`Actor.K2_GetActorLocation` _returnvalue))
  (`self.OnAttackEnded`))

(event `FireBullet`
  (params (TraceStart :type "Vector Structure") (TraceEnd :type "Vector Structure") (DamageInfo :type "/Game/_Core/Utils/S_DammageInfo Structure"))
  ;[0.008875 0.05971 0.3802] Attack bullet
  (bind (_outhits _returnvalue) (`KismetSystemLibrary.LineTraceMultiForObjects` TraceStart TraceEnd (`|MakeArray` "ObjectTypeQuery3" :!type "EObjectTypeQuery Enum") false (`|MakeArray` (`self.GetOwner`)) "ForDuration"))
  (if _returnvalue
    (bind _dammageactor (`self.DamageFirstNonTeamMember` _outhits DamageInfo))
    (`AISense_Damage.ReportDamageEvent` _dammageactor (`self.GetOwner`) (`.Amount_2_372379F2408E17C0DE5E86A6585F6FE9` (break `/Game/_Core/Utils/S_DammageInfo` DamageInfo)) (`Actor.K2_GetActorLocation` (`self.GetOwner`)))))

(event `LightningStrike`
  (params (AttackTarget :type "Actor Object Reference") (DelayBeforeStrike :type "Float (single-precision)") (DamageAmount :type "Float (double-precision)"))
  (bind (_aspawn _bsuccess) (cast `Pawn` (`self.GetOwner`) :!pure true))
  ;[1 1 1] Lightning strike
  (bind _returnvalue (`|SpawnActorFromClass` "/Game/_Core/AOE/BP_AOE_Blast_Lightning.BP_AOE_Blast_Lightning_C" (`KismetMathLibrary.MakeTransform` (0.0 0.0 0.0) (struct) (0.5 0.5 0.5)) "Undefined" "MultiplyWithRoot" null DelayBeforeStrike AttackTarget "/Game/_Core/Decals/Strike_Mat.Strike_Mat" true true false (select `bool` _bsuccess :`true` _aspawn)))
  (add `/Game/_Core/AOE/BP_AOE_Base.OnAOE_OverlapActor` _returnvalue (delegate `OnAOE_PushBackPlayer_Event`)))

(event `OnAOE_PushBackPlayer_Event`
  (params (Actor :type "Actor Object Reference"))
  ;[1 1 1] Lightning strike
  (message `/Game/_Core/Utils/BPI_Dammagable.TakeDamage` Actor (make `/Game/_Core/Utils/S_DammageInfo` (stale `LightningStrike` DamageAmount) "NewEnumerator3" "NewEnumerator1") null))

(event `HealTarget`
  (params (HealTarget :type "Actor Object Reference"))
  (bind _returnvalue (`Actor.K2_GetActorLocation` HealTarget))
  ;[1 1 1] Comment
  (`/Engine/EditorBlueprintResources/StandardMacros.IsValid` HealTarget
    (:`Is Valid`
      (bind (_outhit _returnvalue_2) (`KismetSystemLibrary.LineTraceSingle` _returnvalue (* _returnvalue (0.0 0.0 -1000.0)) "TraceTypeQuery1" false (`|MakeArray` HealTarget)))
      (if _returnvalue_2
        (bind _returnvalue_3 (`|SpawnActorFromClass` "/Game/_Core/AOE/BP_AOE_OverTime_Heal.BP_AOE_OverTime_Heal_C" (`KismetMathLibrary.MakeTransform` (`.Location` (`GameplayStatics.BreakHitResult` _outhit))) "Undefined" "MultiplyWithRoot" null 1.0 10.0 false false false null))
        (add `/Game/_Core/AOE/BP_AOE_Base.OnAOE_OverlapActor` _returnvalue_3 (delegate `OnHealTarget`))
        (`/Game/_Core/AOE/BP_AOE_Base.Trigger` _returnvalue_3)))))

(event `OnHealTarget`
  (params (Actor :type "Actor Object Reference"))
  ;[1 1 1] Comment
  (if (== Actor (stale `HealTarget` HealTarget))
    (message `/Game/_Core/Utils/BPI_Dammagable.Heal` Actor 10.0)))

(event `GroundSmash`
  (params (AttackInfo :type "/Game/_Core/Utils/S_AttackInfo Structure") (Radius :type "Float (single-precision)"))
  (bind (_attacktarget _montage _damageinfo) (break `/Game/_Core/Utils/S_AttackInfo` AttackInfo))
  (bind _returnvalue (`self.GetOwner`))
  ;[0.113 0.1355 0.217] GROUND ROCK ATTACK
  (bind _mesh (`self.AttackBase` _attacktarget))
  (bind _notifyname (`|PlayMontage` _mesh _montage)
    (:`then`
      (message `/Game/_Core/Utils/BPI_Dammagable.SetIsInterruptable` _returnvalue false))
    (:`OnCompleted`
      (message `/Game/_Core/AI/BPI_Enemy_Base_AI.Attack` _returnvalue _attacktarget :!label _label)
      (message `/Game/_Core/Utils/BPI_Dammagable.SetIsInterruptable` _returnvalue true))
    (:`OnInterrupted`
      (goto _label))
    (:`OnNotifyBegin`
      (switch `name` _notifyname
        (:`Smash`
          (`self.AOEDamage` Radius _damageinfo))))))

(event `AOEDamage`
  (params (Radius :type "Float (single-precision)") (DamageInfo :type "/Game/_Core/Utils/S_DammageInfo Structure"))
  (bind _returnvalue (`self.GetOwner`))
  ;[0.224 0.04705 0.1572] AOE Damage
  (`KismetSystemLibrary.PrintString` "aoe damage")
  (bind _returnvalue_2 (`|SpawnActorFromClass` "/Game/_Core/AOE/BP_AOE_Base.BP_AOE_Base_C" (`KismetMathLibrary.MakeTransform` (`Actor.K2_GetActorLocation` _returnvalue)) "Undefined" "MultiplyWithRoot" null true true false (cast `Pawn` _returnvalue :!pure true)))
  (set `/Game/_Core/AOE/BP_AOE_Base.Radius` Radius _returnvalue_2)
  (add `/Game/_Core/AOE/BP_AOE_Base.OnAOE_OverlapActor` _returnvalue_2 (delegate `DamageActorOnEOEActor`))
  (`/Game/_Core/AOE/BP_AOE_Base.Trigger` _returnvalue_2))

(event `DamageActorOnEOEActor`
  (params (Actor :type "Actor Object Reference"))
  (bind _returnvalue (`self.GetOwner`))
  ;[0.224 0.04705 0.1572] AOE Damage
  (bind _teamnumber (message `/Game/_Core/Utils/BPI_Dammagable.GetTeamNumber` Actor))
  (bind _teamnumber_2 (message `/Game/_Core/Utils/BPI_Dammagable.GetTeamNumber` _returnvalue))
  (if (!= _teamnumber_2 _teamnumber)
    (message `/Game/_Core/Utils/BPI_Dammagable.TakeDamage` Actor (stale `AOEDamage` DamageInfo) _returnvalue)))

(event `PrimaryMeleAttaque`
  (params (AttackInfo :type "/Game/_Core/Utils/S_AttackInfo Structure") (Radius :type "Float (single-precision)") (Lengh :type "Float (single-precision)"))
  (bind (_attacktarget _montage _damageinfo) (break `/Game/_Core/Utils/S_AttackInfo` AttackInfo))
  ;[0.07366 0.217 0.107] PRIMARY MELE ATTACK
  (bind _mesh (`self.AttackBase` _attacktarget))
  (bind _notifyname (`|PlayMontage` _mesh _montage)
    (:`OnCompleted`
      (message `/Game/_Core/AI/BPI_Enemy_Base_AI.AttackEnd` (`self.GetOwner`) _attacktarget :!label _label_2))
    (:`OnInterrupted`
      (goto _label_2))
    (:`OnNotifyBegin`
      (switch `name` _notifyname
        (:`Slash`
          (`self.SphereTraceDamage` _damageinfo Radius Lengh))))))

(event `SphereTraceDamage`
  (params (DamageInfo :type "/Game/_Core/Utils/S_DammageInfo Structure") (Radius :type "Float (single-precision)") (Lengh :type "Float (single-precision)" :default 200.0))
  (bind _returnvalue (`self.GetOwner`))
  (bind _returnvalue_2 (`Actor.K2_GetActorLocation` _returnvalue))
  ;[0.224 0.04705 0.1572] SPHERE TRACE
  (bind (_outhits _returnvalue_3) (`KismetSystemLibrary.SphereTraceMultiForObjects` _returnvalue_2 (+ _returnvalue_2 (* Lengh (`Actor.GetActorForwardVector` _returnvalue))) Radius (`|MakeArray` "ObjectTypeQuery3" :!type "EObjectTypeQuery Enum")))
  (if _returnvalue_3
    (`self.DammageAllNonTeamMember` _outhits DamageInfo)))

(event `LongRangeMeleAttack`
  (params (AttackInfo :type "/Game/_Core/Utils/S_AttackInfo Structure"))
  (bind (_attacktarget _montage _damageinfo) (break `/Game/_Core/Utils/S_AttackInfo` AttackInfo))
  (bind _returnvalue (`self.GetOwner`))
  ;[0.113 0.1355 0.217] LONG RANGED ATTACK
  (bind _mesh (`self.AttackBase` _attacktarget))
  (bind _notifyname (`|PlayMontage` _mesh _montage)
    (:`then`
      (message `/Game/_Core/Utils/BPI_Dammagable.SetIsInterruptable` _returnvalue false))
    (:`OnCompleted`
      (message `/Game/_Core/AI/BPI_Enemy_Base_AI.AttackEnd` _returnvalue _attacktarget :!label _label_3)
      (message `/Game/_Core/Utils/BPI_Dammagable.SetIsInterruptable` _returnvalue true))
    (:`OnInterrupted`
      (goto _label_3))
    (:`OnNotifyBegin`
      (switch `name` _notifyname
        (:`Slash`
          (`self.SphereTraceDamage` _damageinfo 20.0))
        (:`Jump`
          (`self.JumpToAttackTarget` _attacktarget))
        (:`AOESlash`
          (`self.AOEDamage` 300.0 _damageinfo))))))

(event `JumpToAttackTarget`
  (params (ActorTarget :type "Actor Object Reference"))
  (bind _returnvalue (`self.GetOwner`))
  (bind _ascharacter (cast `Character` _returnvalue :!pure true))
  ;[0.224 0.04705 0.1572] JUMP TO ATTACK TARGET
  (bind _location (`self.CalculateFutureActorLocation` ActorTarget))
  (bind _outlaunchvelocity (`GameplayStatics.SuggestProjectileVelocity_CustomArc` (`Actor.K2_GetActorLocation` _returnvalue) (`KismetMathLibrary.MakeVector` (.x _location) (.y _location) (+ (.z _location) 100.0)) 0.0 (`KismetMathLibrary.Lerp` 0.5 0.85 (`KismetMathLibrary.FClamp` (`KismetMathLibrary.NormalizeToRange` (`Actor.GetDistanceTo` ActorTarget (`self.GetOwner`)) 400.0 800.0)))))
  (`Character.LaunchCharacter` _ascharacter _outlaunchvelocity true true)
  (add `Character.LandedDelegate` _ascharacter (delegate `AttEnd`)))

(event `AttEnd`
  (params (Hit :type "HitResult Structure (by ref)"))
  (bind _ascharacter (cast `Character` (`self.GetOwner`) :!pure true))
  ;[0.224 0.04705 0.1572] JUMP TO ATTACK TARGET
  (remove `Character.LandedDelegate` _ascharacter (delegate `AttEnd`))
  (`MovementComponent.StopMovementImmediately` (`Character.CharacterMovement` _ascharacter)))

(event `SpinningMeleAttack`
  (params (AttackInfo :type "/Game/_Core/Utils/S_AttackInfo Structure"))
  (bind (_attacktarget _montage _damageinfo) (break `/Game/_Core/Utils/S_AttackInfo` AttackInfo))
  (bind _returnvalue (`self.GetOwner`))
  ;[0.113 0.1355 0.217] Spinning Attack
  (bind _mesh (`self.AttackBase` _attacktarget))
  (bind _notifyname (`|PlayMontage` _mesh _montage)
    (:`then`
      (message `/Game/_Core/Utils/BPI_Dammagable.SetIsInterruptable` _returnvalue false))
    (:`OnCompleted`
      (message `/Game/_Core/AI/BPI_Enemy_Base_AI.AttackEnd` _returnvalue _attacktarget :!label _label_4)
      (message `/Game/_Core/Utils/BPI_Dammagable.SetIsInterruptable` _returnvalue true))
    (:`OnInterrupted`
      (goto _label_4))
    (:`OnNotifyBegin`
      (switch `name` _notifyname
        (:`Slash`
          (`self.SphereTraceDamage` _damageinfo 20.0))
        (:`AOESlash`
          (`self.AOEDamage` 300.0 _damageinfo))))))

(event `BasicMageSpell`
  (params (AttackInfo :type "/Game/_Core/Utils/S_AttackInfo Structure"))
  (bind (_attacktarget _montage _damageinfo) (break `/Game/_Core/Utils/S_AttackInfo` AttackInfo))
  ;[0.113 0.1355 0.217] Basic Magic Spell
  (bind _mesh (`self.AttackBase` _attacktarget))
  (bind _notifyname (`|PlayMontage` _mesh _montage)
    (:`OnCompleted`
      (message `/Game/_Core/AI/BPI_Enemy_Base_AI.AttackEnd` (`self.GetOwner`) _attacktarget :!label _label_5))
    (:`OnInterrupted`
      (goto _label_5))
    (:`OnNotifyBegin`
      (switch `name` _notifyname
        (:`FireBall`
          (`self.MagicSpell` (`KismetMathLibrary.MakeTransform` (`SceneComponent.GetSocketLocation` _mesh "hand_rAttack")) _attacktarget _damageinfo))))))

(event `BarrageMagicSpell`
  (params (AttackInfo :type "/Game/_Core/Utils/S_AttackInfo Structure"))
  (bind (_attacktarget _montage _damageinfo) (break `/Game/_Core/Utils/S_AttackInfo` AttackInfo))
  (bind _returnvalue (`self.GetOwner`))
  ;[0.113 0.1355 0.217] BARRAGE ATTAQUE
  (bind _mesh (`self.AttackBase` _attacktarget))
  (bind _notifyname (`|PlayMontage` _mesh _montage)
    (:`OnCompleted`
      (message `/Game/_Core/AI/BPI_Enemy_Base_AI.AttackEnd` _returnvalue _attacktarget :!label _label_6)
      (message `/Game/_Core/Utils/BPI_Dammagable.SetIsInterruptable` _returnvalue true))
    (:`OnInterrupted`
      (goto _label_6))
    (:`OnNotifyBegin`
      (switch `name` _notifyname
        (:`Fire`
          (`self.MagicSpell` (`KismetMathLibrary.MakeTransform` (`SceneComponent.GetSocketLocation` _mesh "hand_rAttack") (`KismetMathLibrary.FindLookAtRotation` (`Actor.K2_GetActorLocation` (`self.GetOwner`)) (+ (`Actor.K2_GetActorLocation` _attacktarget) (`KismetMathLibrary.MakeVector` 0.0 (`KismetMathLibrary.RandomFloatInRange` -300.0 300.0))))) null _damageinfo true)
          (message `/Game/_Core/Utils/BPI_Dammagable.SetIsInterruptable` _returnvalue false))))))

(event `SimpleAttack`
  (params (InSkeletalMeshComponent :type "SkeletalMeshComponent Object Reference"))
  ;[0.09898 0.5447 1] ATTACK MULTI COMBO  (  SIMPLE  )
  (if (`self.CanAttack?`)
    (set `self.CanAttack?` false)
    (bind _notifyname (`|PlayMontage` InSkeletalMeshComponent (`|GetArrayItem` (`self.ListAttack`) (`self.AtkCount`)))
      (:`OnNotifyBegin`
        (switch `name` _notifyname
          (:`SaveAttack`
            (`self.ValidateAttack`)
            (bind _listeactortouche (`self.TriggerSimple`))
            (for _array_element _listeactortouche
              (message `/Game/_Core/Utils/BPI_Dammagable.TakeDamage` _array_element (make `/Game/_Core/Utils/S_DammageInfo` 10.0 "NewEnumerator1" "NewEnumerator1" false true true) null)))
          (:`ResetCombo`
            (`self.ResetCombo`)))))))

(event `ResetCombo`
  ;[0.09898 0.5447 1] ATTACK MULTI COMBO  (  SIMPLE  )
  (set `self.AtkCount` 0)
  (set `self.CanAttack?` true))

(event `ValidateAttack`
  ;[0.09898 0.5447 1] ATTACK MULTI COMBO  (  SIMPLE  )
  (set `self.CanAttack?` true)
  (if (>= (`self.AtkCount`) (`KismetArrayLibrary.Array_Length` (`self.ListAttack`)))
    (set `self.AtkCount` 0)
    (else
      (`/Engine/EditorBlueprintResources/StandardMacros.IncrementInt` (`self.AtkCount`)))))

(fn `AttackBase`
  (params (AttackTarget :type "Actor Object Reference"))
  (returns (Mesh :type "SkeletalMeshComponent Object Reference"))
  (bind _returnvalue (`self.GetOwner`))
  (message `/Game/_Core/AI/BPI_Enemy_Base_AI.Attack` _returnvalue AttackTarget)
  (bind _ascharacter (cast `Character` _returnvalue))
  (return (`Character.Mesh` _ascharacter)))

(fn `CalculateFutureActorLocation`
  (params (Actor :type "Actor Object Reference") (Time :type "Float (double-precision)" :default 1.0))
  (returns (Location :type "Vector Structure"))
  ;[0.113 0.1355 0.217] Location est la velocite x current location
  (return (+ (`Actor.K2_GetActorLocation` Actor) (* (* (`Actor.GetVelocity` Actor) (1.0 1.0 0.0)) Time))))

(fn `DamageFirstNonTeamMember`
  (params (Hits :type "Array of HitResult Structure") (DamageInfo :type "/Game/_Core/Utils/S_DammageInfo Structure"))
  (returns (DammageActor :type "Actor Object Reference"))
  (bind _returnvalue (`self.GetOwner`))
  (for _array_element Hits
    (bind (_bblockinghit _binitialoverlap _time _distance _location _impactpoint _normal _impactnormal _physmat _hitactor) (`GameplayStatics.BreakHitResult` _array_element))
    (bind _teamnumber (message `/Game/_Core/Utils/BPI_Dammagable.GetTeamNumber` _hitactor))
    (bind _teamnumber_2 (message `/Game/_Core/Utils/BPI_Dammagable.GetTeamNumber` _returnvalue))
    (if (!= _teamnumber_2 _teamnumber)
      (message `/Game/_Core/Utils/BPI_Dammagable.TakeDamage` _hitactor DamageInfo _returnvalue)
      (`|ExecutionSequence`
        (:`then_0`
          (break))
        (:`then_1`
          (return _hitactor))))))

(fn `DammageAllNonTeamMember`
  (params (Hits :type "Array of HitResult Structure") (DamageInfo :type "/Game/_Core/Utils/S_DammageInfo Structure"))
  (returns (ActorsDammaged :type "Array of Actor Object Reference"))
  (locals (ActorDammageSoFar :type "Array of Actor Object Reference"))
  (bind _returnvalue (`self.GetOwner`))
  (for _array_element Hits
    (bind (_bblockinghit _binitialoverlap _time _distance _location _impactpoint _normal _impactnormal _physmat _hitactor) (`GameplayStatics.BreakHitResult` _array_element))
    (bind _teamnumber (message `/Game/_Core/Utils/BPI_Dammagable.GetTeamNumber` _hitactor))
    (bind _teamnumber_2 (message `/Game/_Core/Utils/BPI_Dammagable.GetTeamNumber` _returnvalue))
    (if (and (!= _teamnumber_2 _teamnumber) (not (`KismetArrayLibrary.Array_Contains` (`local.ActorDammageSoFar`) _hitactor)))
      (message `/Game/_Core/Utils/BPI_Dammagable.TakeDamage` _hitactor DamageInfo _returnvalue)
      (`KismetArrayLibrary.Array_AddUnique` (`local.ActorDammageSoFar`) _hitactor)))
  (return (`local.ActorDammageSoFar`)))

(fn `FillAttackList`
  (params (ListAttack :type "Array of AnimMontage Object Reference"))
  (set `self.ListAttack` ListAttack)
  (`KismetSystemLibrary.PrintString` "List attaque completed"))

(fn `TriggerComplexeHit`
  (params (TraceStart :type Name) (TraceEnd :type Name) (AttackTarget :type "Actor Object Reference"))
  (bind _ascharacter (cast `Character` AttackTarget :!pure true))
  (bind (_outhit _returnvalue) (`KismetSystemLibrary.SphereTraceSingleForObjects` :`Start` (`SceneComponent.GetSocketLocation` (`Actor.RootComponent` _ascharacter) TraceStart) :`End` (`SceneComponent.GetSocketLocation` (`Actor.RootComponent` _ascharacter) TraceEnd) :`Radius` 5.0 :`ObjectTypes` (`|MakeArray` "ObjectTypeQuery3" :!type "EObjectTypeQuery Enum") :`DrawDebugType` "ForDuration"))
  (if _returnvalue
    (`KismetSystemLibrary.PrintString` "on a un hit")))

(fn `TriggerSimple`
  (returns (ListeActorTouche :type "Array of Actor Object Reference"))
  (bind _returnvalue (`self.GetOwner`))
  (bind _returnvalue_2 (`Actor.GetActorForwardVector` _returnvalue))
  (bind (_outhits _returnvalue_3) (`KismetSystemLibrary.BoxTraceMultiForObjects` :`Start` (`Actor.K2_GetActorLocation` _returnvalue) :`End` (+ (`Actor.K2_GetActorLocation` _returnvalue) (* _returnvalue_2 120.0)) :`HalfSize` (100.0 100.0 50.0) :`Orientation` (`KismetMathLibrary.Conv_VectorToRotator` _returnvalue_2) :`ObjectTypes` (`|MakeArray` "ObjectTypeQuery3" :!type "EObjectTypeQuery Enum") :`bTraceComplex` true :`DrawDebugType` "ForDuration"))
  (for _array_element _outhits
    (if _returnvalue_3
      (`KismetArrayLibrary.Array_AddUnique` (`self.ListeActorTouche`) (`.HitActor` (`GameplayStatics.BreakHitResult` _array_element)))))
  (return (`self.ListeActorTouche`)))