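; BP_EnemySpawner is a spawner actor that places BP_Enemy_Base AI enemies at random points inside its EnemiesSpawnZone box.
; It registers itself with the game mode on BeginPlay so the game mode can control it.
; Each SpawnOneEnemy call asks the game mode for permission, spawns one enemy if allowed, then tells the game mode to increment its enemy count.
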(event `self.ReceiveBeginPlay`
  ;[0.04924 0.01331 0.1875] demande au game mode d'enregistrer ce spawner pour pouvoir le controler
  (message `/Game/_Core/BPI_GameMode_MP.RegisterSpawner` (`GameplayStatics.GetGameMode`) self))

(event `SpawnOneEnemy`
  (bind _enemiesspawnzone (`self.EnemiesSpawnZone`))
  ;[0.002024 0.000566 0.02604] Spawn un enemy a un endroit aleatoire dans la box
  (bind _result (message `/Game/_Core/BPI_GameMode_MP.CanSpawnOneEnemy` (`GameplayStatics.GetGameMode`))) ; demande au game mode de faire spawn
  (if _result
    (`AIBlueprintHelperLibrary.SpawnAIFromClass` "/Game/_Core/Character/Enemy/BP_Enemy_Base.BP_Enemy_Base_C" null (`KismetMathLibrary.RandomPointInBoundingBox` (`SceneComponent.K2_GetComponentLocation` _enemiesspawnzone) (`BoxComponent.GetScaledBoxExtent` _enemiesspawnzone)) (struct) false null)
    (message `/Game/_Core/BPI_GameMode_MP.IncrementEnemyCount` (`GameplayStatics.GetGameMode`)) ; Previens le game mode qu'in enemy a été spawn
  ))

(fn `UserConstructionScript`)