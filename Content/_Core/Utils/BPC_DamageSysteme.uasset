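; Damage system component that holds an actor's health, stamina, XP/level and attack token pool.
; TakeDamage uses the CanBeDammaged macro to filter death, invincibility and blocking, then fires block, death or interruptible damage-response dispatchers for the owner.
; Attack tokens are reserved and returned by amount, and filling XP levels up with a higher threshold and a sound.
; FindHealthToDelete is an unfinished stub returning zero.
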(fn `DecreaseStamina`
  (params (StaminaDepleted :type "Float (double-precision)"))
  (returns (`Not Stamina Left` :type Boolean))
  (set `self.IsStaminaFull?` false)
  (if (not (<= (`self.CurrentStamina`) 0.0))
    (set `self.CurrentStamina` (- (`self.CurrentStamina`) StaminaDepleted))
    (if (<= (`self.CurrentStamina`) 0.0)
      _
      (else
        (return false))))
  (return true))

(fn `FindHealthToDelete`
  (params (HealthReceive :type "Float (double-precision)"))
  (returns (NewHealth :type "Float (double-precision)"))
  ;[1 0 0.01161] A COMPLETER
  (return 0.0))

(fn `Heal`
  (params (Amount :type "Float (double-precision)"))
  (returns (NewHealth :type "Float (double-precision)"))
  (if (not (`self.IsDead?`))
    (bind _output_get (set `self.CurrentHealth` (`KismetMathLibrary.FClamp` (+ Amount (`self.CurrentHealth`)) 0.0 (`self.MaxHealth`))))
    (return _output_get)))

(fn `IncreaseLevel`
  (params (AddedLevel :type Integer))
  (set `self.CurrentLevel` (+ AddedLevel (`self.CurrentLevel`)))
  (set `self.MaxXP` (+ (`self.MaxXP`) 150.0))
  (set `self.CurrentXP` 0.0)
  (`GameplayStatics.PlaySound2D` "/Game/_Core/Sound/UI/LevelUp1.LevelUp1" 1.0 1.0 0.0 null null))

(fn `IncreaseMaxHealth`
  (params (NewMaxHealth :type "Float (double-precision)"))
  (bind _output_get (set `self.MaxHealth` (+ (`self.MaxHealth`) NewMaxHealth)))
  (set `self.CurrentHealth` _output_get))

(fn `IncreaseMaxStamina`
  (params (AddStamina :type "Float (double-precision)"))
  (set `self.MaxStamina` (+ (`self.MaxStamina`) AddStamina)))

(fn `IncreaseStamina`
  (params (AddedStamina :type "Float (double-precision)"))
  (set `self.CurrentStamina` (+ AddedStamina (`self.CurrentStamina`)))
  (if (> (`self.CurrentStamina`) (`self.MaxStamina`))
    (set `self.CurrentStamina` (`self.MaxStamina`))
    (else
      (set `self.IsStaminaFull?` true))))

(fn `IncreaseXP`
  (params (AddedXP :type "Float (double-precision)"))
  (set `self.CurrentXP` (+ AddedXP (`self.CurrentXP`)))
  (if (>= (`self.CurrentXP`) (`self.MaxXP`))
    (`self.IncreaseLevel` 1)))

(fn `ReserveAttackToken`
  (params (Amount :type Integer))
  (returns (Succes :type Boolean))
  (if (>= (`self.AttackTokenCount`) Amount)
    (set `self.AttackTokenCount` (- (`self.AttackTokenCount`) Amount))
    (return true)
    (else
      (return false))))

(fn `ReturnAttackToken`
  (params (Amount :type Integer))
  (set `self.AttackTokenCount` (+ (`self.AttackTokenCount`) Amount)))

(fn `TakeDamage`
  (params (DamageInfo :type "/Game/_Core/Utils/S_DammageInfo Structure") (DamageCauser :type "Actor Object Reference"))
  (returns (WasDamaged :type Boolean))
  (bind (_amount _dammagetype _dammageresponse _shoulddammadeinvincible _canbeblock _canbeparry _shouldforceinterrupt) (break `/Game/_Core/Utils/S_DammageInfo` DamageInfo))
  (`self.CanBeDammaged` _shoulddammadeinvincible _canbeblock
    (:`BlockDamage`
      (`self.OnBlock` _canbeparry DamageCauser)
      (return false))
    (:`DoDamage`
      (bind _output_get (set `self.CurrentHealth` (- (`self.CurrentHealth`) _amount)))
      (if (<= _output_get 0.0)
        (set `self.IsDead?` true)
        (`self.OnDeath`)
        (elif (or (`self.IsInterruptible?`) _shouldforceinterrupt)
          (`self.OnDammageResponse` _dammageresponse DamageCauser)))
      (return true))))