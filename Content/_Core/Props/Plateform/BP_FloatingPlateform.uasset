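; Floating platform prop that rises vertically from its starting position shortly after play begins.
; StartFloating stores the current Z, then plays a Timeline that lerps the actor up by a fixed height while keeping X and Y.
; StopFloating reverses the same Timeline to lower it back, and the Timeline's Finished output calls the OnFloatTimelineFinished dispatcher.
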(event `self.ReceiveBeginPlay`
  (`KismetSystemLibrary.Delay` 0.5)
  (`self.StartFloating`))

(event `StartFloating`
  (bind (_returnvalue_x _returnvalue_y _returnvalue_z) (`KismetMathLibrary.BreakVector` (`self.K2_GetActorLocation`)))
  (bind _initialzvalue (`self.InitialZValue`))
  (set `self.InitialZValue` _returnvalue_z)
  (bind (_direction _alphaz) (`Timeline|Timeline` :!label _label)
    (:`Update`
      (`self.K2_SetActorLocation` (`KismetMathLibrary.MakeVector` _returnvalue_x _returnvalue_y (`KismetMathLibrary.Lerp` _initialzvalue (+ _initialzvalue 350.0) _alphaz))))
    (:`Finished`
      (`self.OnFloatTimelineFinished`))))

(event `StopFloating`
  (goto _label :!via `Reverse`))

(fn `UserConstructionScript`)