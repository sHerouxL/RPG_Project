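; Game mode blueprint that tracks the live enemy count against a maximum and handles player respawn and spawner registration.
; Registering a spawner starts a looping timer at the enemies-per-second rate, and Tick prints the count on screen.
; RespawnPlayer spawns BP_EnemySpawner at the stored player transform, despite its hero comment, then calls Possess.
; Health and score UI events are empty, their widget logic left disconnected.
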(event `self.ReceiveBeginPlay`
  ;[0.01514 0.000851 0.03472] creer le widget qui affiche la barre de vie et score et ajoute a ecran
)

(event `RespawnPlayer`
  ;[0.1719 0.008559 0.1298] Fait apparaitre une copie du hero et donne le controle de cette derniere au player
  (`|SpawnActorFromClass` "/Game/_Core/Utils/BP_EnemySpawner.BP_EnemySpawner_C" (`self.PlayerSpawnTransform`) "Undefined" "MultiplyWithRoot" null null)
  (`Controller.Possess` (`GameplayStatics.GetPlayerController` 0) null))

(event `/Game/_Core/BPI_GameMode_MP.RegisterSpawner`
  (params (NewSpawner :type "/Game/_Core/Utils/BP_EnemySpawner Object Reference"))
  ;[0.000792 0.01306 0.04167] Enregistre le spawner place dans le monde et demande de faire spawn enemy
  (bind _output_get (set `self.EnemySpawner` NewSpawner))
  (`KismetSystemLibrary.K2_SetTimerDelegate` (`|CreateDelegate` _output_get :!event `SpawnOneEnemy`) (/ 1.0 (`self.EnemyPerSeconde`)) true))

(event `/Game/_Core/BPI_GameMode_MP.IncrementEnemyCount`
  ;[0.01514 0.000851 0.03472] Met a jour le compteur en fonction du nombre d'enemy sur la map
  (`/Engine/EditorBlueprintResources/StandardMacros.IncrementInt` (`self.CurrentEnemyCount`)))

(event `/Game/_Core/BPI_GameMode_MP.DecrementEnemyCount`
  ;[0.01514 0.000851 0.03472] Met a jour le compteur en fonction du nombre d'enemy sur la map
  (`/Engine/EditorBlueprintResources/StandardMacros.DecrementInt` (`self.CurrentEnemyCount`)))

(event `self.ReceiveTick`
  (params (DeltaSeconds :type "Float (single-precision)"))
  ;[0.01514 0.000851 0.03472] affiche le nombre d'ennemy actuellement en jeux
  (`KismetSystemLibrary.PrintString` (`KismetStringLibrary.Concat_StrStr` "Nombre ennemy = " (`KismetStringLibrary.Conv_IntToString` (`self.CurrentEnemyCount`))) true true (struct :`R` 0.322917 :`G` 0.297824 :`B` 0.030815 :`A` 1.0) 0.0))

(event `/Game/_Core/BPI_GameMode_MP.UpdateUI_PlayerHealth`
  (params (NewHealth :type "Float (double-precision)"))
  ;[0.01514 0.000851 0.03472] Met a jour la barre de vie du joueur
)

(event `/Game/_Core/BPI_GameMode_MP.UpdateUI_Score`
  ;[0.01514 0.000851 0.03472] Met a jour le score et l'envoie au widget
)

(fn `CanSpawnOneEnemy`
  (returns (Result :type Boolean))
  ;[0.08333 0.004269 0.02961] on ne peut spawn des ennemy que si on n'a pas atteint le nombre max
  (return (< (`self.CurrentEnemyCount`) (`self.MaxEnemyCount`))))

(fn `GetEnemyCount`
  (returns (EnemyCount :type Integer))
  ;[0.2529 0.09399 1] recupere le nombre d'ennemy sur la map
  (return (`self.CurrentEnemyCount`)))

(fn `SetPlayerSpawnTransform`
  (params (PlayerSpawnTransform :type "Transform Structure"))
  ;[0.08558 0.3564 1] stock la position de depart du player
  (set `self.PlayerSpawnTransform` PlayerSpawnTransform)
  (return))

(fn `UserConstructionScript`)