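; BP_Dummy is a stealth assassination target that plays the victim side of a paired knife kill.
; An overlap radius toggles an assassination prompt widget for BP_Player, which Tick rotates to face the camera.
; StealthBackAssasin plays the victim montage, hides the prompt and returns the AssasineRef location with the dummy's rotation to the caller.
; It also triggers a delayed switch of the mesh to ragdoll physics.
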(event `self.ReceiveBeginPlay`)

(event `self.ReceiveTick`
  (params (DeltaSeconds :type "Float (single-precision)"))
  (`SceneComponent.K2_SetWorldRotation` (`self.AssasinateWidget`) (`KismetMathLibrary.FindLookAtRotation` (`SceneComponent.K2_GetComponentLocation` (`self.AssasinateWidget`)) (`SceneComponent.K2_GetComponentLocation` (`PlayerCameraManager.TransformComponent` (`GameplayStatics.GetPlayerCameraManager` 0)))) false false))

(event `Ragdoll`
  ;[0.05127 0.05127 0.05127] ragdoll
  (`KismetSystemLibrary.Delay` 2.3)
  (`PrimitiveComponent.SetSimulatePhysics` (`self.Mesh`) true))

(event `self.AssasineRadius.OnComponentBeginOverlap`
  (params (OverlappedComponent :type "PrimitiveComponent Object Reference") (OtherActor :type "Actor Object Reference") (OtherComp :type "PrimitiveComponent Object Reference") (OtherBodyIndex :type Integer) (bFromSweep :type Boolean) (SweepResult :type "HitResult Structure (by ref)"))
  ;[0.05127 0.05127 0.05127] affichage widget assasination on / off
  (cast `/Game/_GameMain/RPJ_Character/BP_Player` OtherActor)
  (`SceneComponent.SetVisibility` (`self.AssasinateWidget`) true false))

(event `self.AssasineRadius.OnComponentEndOverlap`
  (params (OverlappedComponent :type "PrimitiveComponent Object Reference") (OtherActor :type "Actor Object Reference") (OtherComp :type "PrimitiveComponent Object Reference") (OtherBodyIndex :type Integer))
  ;[0.05127 0.05127 0.05127] affichage widget assasination on / off
  (cast `/Game/_GameMain/RPJ_Character/BP_Player` OtherActor)
  (`SceneComponent.SetVisibility` (`self.AssasinateWidget`) false false))

(fn `StealthBackAssasin`
  (returns (RefLocation :type "Vector Structure") (RefRotation :type "Rotator Structure"))
  (`self.PlayAnimMontage` "/Game/_GameMain/RPJ_Character/Animation/Assasination/Paired_Knife_Stealth_KidneyAndNeck_Vic_Montage.Paired_Knife_Stealth_KidneyAndNeck_Vic_Montage")
  (`self.Ragdoll`)
  (`SceneComponent.SetVisibility` (`self.AssasinateWidget`) false false)
  (return (`SceneComponent.K2_GetComponentLocation` (`self.AssasineRef`)) (`self.K2_GetActorRotation`)))

(fn `UserConstructionScript`)